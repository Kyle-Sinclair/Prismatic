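; Volumetric fog Blueprint, named for the main menu, that fakes a volume by stacking static mesh layers at BeginPlay.
; A loop driven by VolumeResolution adds meshes at increasing relative Z, spaced by VolumeHeight divided by the resolution.
; The base Plane gets a dynamic material fed its world Z and VolumeHeight, though the minimum parameter name reads "NoneMinFrom_BP".
; Matching material setup for the added layers exists but never runs.
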(event EventBeginPlay
  (bind _plane (Variables|Default|GetPlane))
  (bind _returnvalue (Transformation|GetWorldLocation _plane))
  (bind _returnvalue_2 (Rendering|Material|CreateDynamicMaterialInstance _plane 0 (Rendering|Material|GetMaterial (Variables|Default|GetPlane) 0) "None" :!class /Script/Engine.PrimitiveComponent))
  (Variables|Default|SetSeedHeight (.z _returnvalue))
  (Rendering|Material|SetScalarParameterValue _returnvalue_2 "NoneMinFrom_BP" (.z _returnvalue) :!class /Script/Engine.MaterialInstanceDynamic)
  (Rendering|Material|SetScalarParameterValue _returnvalue_2 "MaxFrom_BP" (Variables|Default|GetVolumeHeight) :!class /Script/Engine.MaterialInstanceDynamic)
  (for _index (range 0 (Variables|Default|GetVolumeResolution))
    (bind _returnvalue_3 (AddComponent|AddStaticMeshComponent false (Math|Transform|MakeTransform (Math|Vector|MakeVector 0.0 0.0 (+ (Variables|Default|GetPreviousLayerHeight) (/ (Variables|Default|GetVolumeHeight) (Math|Conversions|ToByte(Integer) (Variables|Default|GetVolumeResolution))))) "0, 0, 0" "1.000000,1.000000,1.000000")))
    (Variables|Default|SetPreviousLayerHeight (+ (Variables|Default|GetPreviousLayerHeight) (/ (Variables|Default|GetVolumeHeight) (Math|Conversions|ToByte(Integer) (Variables|Default|GetVolumeResolution)))))))

(fn ConstructionScript)