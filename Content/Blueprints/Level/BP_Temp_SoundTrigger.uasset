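; BP_Temp_SoundTrigger is a level trigger that fires a one-time dialogue when the player character overlaps it.
; The Game Instance tracks which message IDs are used, so an unused ID is marked and then passed by name to BPOnCollisionComponent's OnDialogueTriggered.
; The construction script hides the trigger component in game unless Debug is enabled.
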(event EventTick
  (params (DeltaSeconds :type Float%20%28single-precision%29)))

(event Collision|EventActorBeginOverlap
  (params (OtherActor :type Actor%20Object%20Reference))
  (bind _id (Variables|Default|GetID))
  ;[1 1 1] Comment
  (if (== OtherActor (Game|GetPlayerCharacter 0))
    (bind _isused (Class|DialogueManagerBPI|GetRowIndexUsed(Message) (Game|GetGameInstance) _id))
    (if (not _isused)
      (Class|DialogueManagerBPI|SetRowIndexUsed(Message) (Game|GetGameInstance) (Variables|Default|GetID))
      (Default|OnDialogueTriggered (Variables|Default|GetBP_OnCollisionComponent) (Utilities|String|StringToName (Utilities|String|EnumtoString _id))))))

(fn ConstructionScript
  (Development|SetHiddeninGame (Variables|Default|GetTrigger) (not (Variables|Default|GetDebug)) false))