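; Kill tunnel trap puzzle that moves walls in on the player and kills them through the resurrection manager unless they reach safety.
; Overlap triggers rotate doors and enable an invisible wall, start the walls, change their speed, flag the player safe and handle crash audio.
; After a death, a timer resets walls, doors, state and the breakable wall spawner, re-arming the DoOnce gates on kill, door, audio and crash FX.
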(event OnComponentBeginOverlap(Trigger_TrapActivate)
  (params (OverlappedComponent :type Primitive%20Component%20Object%20Reference) (OtherActor :type Actor%20Object%20Reference) (OtherComp :type Primitive%20Component%20Object%20Reference) (OtherBodyIndex :type Integer) (bFromSweep :type Boolean) (SweepResult :type Hit%20Result%20Structure%20%28by%20ref%29))
  (Utilities|Casting|CastToCharacter OtherActor)
  (if (Utilities|Array|IsValidIndex (Variables|Default|GetKillTunnelWalls))
    (Variables|Default|SetTrapActivated true)
    (bind _returnvalue (Audio|SpawnSoundatLocation "/Game/Audio/Level/Kill_Tunnel/KT_Wall_Closing__Cue.KT_Wall_Closing__Cue" (Transformation|GetActorLocation) "0, 0, 0" 1.0 1.0 0.0 0 0))
    (Variables|Default|SetAudioWallMoving _returnvalue)
    (for _array_element (Variables|Default|GetKillTunnelWalls)
      (Default|MoveWall _array_element)
      (Default|PlayMoveFX _array_element))))

(event OnComponentBeginOverlap(Trigger_TrapSpeed)
  (params (OverlappedComponent :type Primitive%20Component%20Object%20Reference) (OtherActor :type Actor%20Object%20Reference) (OtherComp :type Primitive%20Component%20Object%20Reference) (OtherBodyIndex :type Integer) (bFromSweep :type Boolean) (SweepResult :type Hit%20Result%20Structure%20%28by%20ref%29))
  (Utilities|Casting|CastToCharacter OtherActor)
  (for _array_element (Variables|Default|GetKillTunnelWalls)
    (Components|Timeline|SetPlayRate (Variables|/Game/Blueprints/Level/KillTunnel/BP_KillTunnelWall.BP_KillTunnelWall_C|GetTimeline _array_element) (/ 1.0 (/ (Variables|/Game/Blueprints/Level/KillTunnel/BP_KillTunnelWall.BP_KillTunnelWall_C|GetTrapDuration _array_element) (Variables|Default|GetSpeedMultiplier))))))

(event OnComponentBeginOverlap(Trigger_Kill)
  (params (OverlappedComponent :type Primitive%20Component%20Object%20Reference) (OtherActor :type Actor%20Object%20Reference) (OtherComp :type Primitive%20Component%20Object%20Reference) (OtherBodyIndex :type Integer) (bFromSweep :type Boolean) (SweepResult :type Hit%20Result%20Structure%20%28by%20ref%29))
  (Utilities|Casting|CastToBP_KillTunnelWall OtherActor)
  (Utilities|FlowControl|DoOnce false
    (:Completed
      (if (not (Variables|Default|GetbPlayerSafe))
        (Audio|PlaySoundatLocation "/Game/Audio/Character/Death/Death_Wall__Cue.Death_Wall__Cue" (Transformation|GetActorLocation OtherActor) "0, 0, 0" 1.0 1.0 0.0 0 0 0 0)
        (Class|ResurrectionManager|TryKillPlayer (Variables|Default|GetResManager))
        (Utilities|Time|SetTimerbyEvent (delegate Custom|ResetPuzzle) (Variables|Default|GetResetDelayTime))))))

(event OnComponentBeginOverlap(Trigger_Doors)
  (params (OverlappedComponent :type Primitive%20Component%20Object%20Reference) (OtherActor :type Actor%20Object%20Reference) (OtherComp :type Primitive%20Component%20Object%20Reference) (OtherBodyIndex :type Integer) (bFromSweep :type Boolean) (SweepResult :type Hit%20Result%20Structure%20%28by%20ref%29))
  (Utilities|Casting|CastToCharacter OtherActor)
  (Utilities|FlowControl|DoOnce false
    (:Completed
      (Collision|SetCollisionEnabled (Variables|Default|GetInvisibleWall) "QueryAndPhysics")
      (for _array_element (Variables|Default|GetKillTunnelDoors)
        (Default|RotateDoor _array_element))
      (for _array_element_2 (Variables|Default|GetKillTunnelWalls)
        (Default|PlayWakeUpFX _array_element_2)))))

(event OnComponentBeginOverlap(Trigger_PlayerSafe)
  (params (OverlappedComponent :type Primitive%20Component%20Object%20Reference) (OtherActor :type Actor%20Object%20Reference) (OtherComp :type Primitive%20Component%20Object%20Reference) (OtherBodyIndex :type Integer) (bFromSweep :type Boolean) (SweepResult :type Hit%20Result%20Structure%20%28by%20ref%29))
  (Utilities|Casting|CastToCharacter OtherActor)
  (if (Variables|Default|GetTrapActivated)
    (Variables|Default|SetbPlayerSafe true)
    (Variables|Default|SetTrapActivated false)))

(event OnComponentBeginOverlap(Trigger_CloseAudio)
  (params (OverlappedComponent :type Primitive%20Component%20Object%20Reference) (OtherActor :type Actor%20Object%20Reference) (OtherComp :type Primitive%20Component%20Object%20Reference) (OtherBodyIndex :type Integer) (bFromSweep :type Boolean) (SweepResult :type Hit%20Result%20Structure%20%28by%20ref%29))
  (Utilities|Casting|CastToBP_KillTunnelWall OtherActor)
  (Utilities|FlowControl|DoOnce false
    (:Completed
      (Audio|PlaySoundatLocation "/Game/Audio/Level/Kill_Tunnel/KT_Wall_Crash_Cue.KT_Wall_Crash_Cue" (Transformation|GetActorLocation) "0, 0, 0" 1.0 1.0 0.0 0 0 0 0)
      (Audio|Components|Audio|FadeOut (Variables|Default|GetAudioWallMoving) 1.2 0.0 "Linear" :!class /Script/Engine.AudioComponent))))

(event Custom|ResetPuzzle
  (Utilities|FlowControl|Sequence
    (:then_0
      (for _array_element (Variables|Default|GetKillTunnelWalls)
        (Audio|Components|Audio|Stop (Variables|/Game/Blueprints/Level/KillTunnel/BP_KillTunnelWall.BP_KillTunnelWall_C|GetTimeline _array_element))
        (Components|Timeline|SetNewTime (Variables|/Game/Blueprints/Level/KillTunnel/BP_KillTunnelWall.BP_KillTunnelWall_C|GetTimeline _array_element) 0.0)
        (Transformation|SetActorLocation _array_element (Variables|/Game/Blueprints/Level/KillTunnel/BP_KillTunnelWall.BP_KillTunnelWall_C|GetStartLocation _array_element) false true)
        (CallFunction|ResetKillTrigger)
        (CallFunction|ResetDoorTrigger)
        (CallFunction|ResetCloseTrigger)
        (Default|ResetVFX _array_element)))
    (:then_1
      (for _array_element_2 (Variables|Default|GetKillTunnelDoors)
        (Audio|Components|Audio|Stop (Variables|/Game/Blueprints/Level/KillTunnel/BP_KillTunnelDoor.BP_KillTunnelDoor_C|GetRotationTimeline _array_element_2))
        (Components|Timeline|SetNewTime (Variables|/Game/Blueprints/Level/KillTunnel/BP_KillTunnelDoor.BP_KillTunnelDoor_C|GetRotationTimeline _array_element_2) 0.0)
        (Transformation|SetActorRotation _array_element_2 (Variables|/Game/Blueprints/Level/KillTunnel/BP_KillTunnelDoor.BP_KillTunnelDoor_C|GetStartRotation _array_element_2) true)))
    (:then_2
      (Collision|SetCollisionEnabled (Variables|Default|GetInvisibleWall) "NoCollision")
      (Variables|Default|SetbPlayerSafe false)
      (Variables|Default|SetTrapActivated false))
    (:then_3
      (Default|RespawnActor (Variables|Default|GetBreakableWallSpawner))
      (CallFunction|ResetCrashFX))))

(event Custom|ResetKillTrigger
  (Utilities|FlowControl|DoOnce false) ; enters at Reset
)

(event Custom|ResetDoorTrigger
  (Utilities|FlowControl|DoOnce false) ; enters at Reset
)

(event Custom|ResetCloseTrigger
  (Utilities|FlowControl|DoOnce false) ; enters at Reset
)

(event Custom|PlayCrashFX
  ;[1 1 1] Reset Crash FX
  (Utilities|FlowControl|DoOnce false
    (:Completed
      (Components|Activation|Activate (Variables|Default|GetNiagara_CrashFX) true))))

(event Custom|ResetCrashFX
  ;[1 1 1] Reset Crash FX
  (Utilities|FlowControl|DoOnce false) ; enters at Reset
)

(event EventBeginPlay
  (Collision|SetCollisionEnabled (Variables|Default|GetInvisibleWall) "NoCollision")
  ;[1 1 1] Get Reference To Res System
  (bind _asbp_gp3game_mode (Utilities|Casting|CastToBP_GP3GameMode (Game|GetGameMode)))
  (bind _asbp_resurrection_manager (Utilities|Casting|CastToBP_ResurrectionManager (Class|GP3GameMode|GetResManager _asbp_gp3game_mode))
    (:then
      (Variables|Default|SetResManager _asbp_resurrection_manager))
    (:CastFailed
      (Development|PrintString "KillTunnel failed to get a reference to the resurrection system"))))

(fn ConstructionScript)