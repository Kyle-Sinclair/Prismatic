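; BP_KillTunnelDoor is a kill tunnel door actor that swings shut by rotating around its yaw axis.
; On BeginPlay it stores its starting rotation.
; RotateDoor plays a closing sound and runs a curve-driven timeline, with play rate set from CloseDuration, that lerps yaw from the start value to ClosedRotationZ while preserving roll and pitch.
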(event Custom|RotateDoor
  (bind _startrotation (Variables|Default|GetStartRotation))
  (Audio|PlaySoundatLocation "/Game/Audio/Level/Kill_Tunnel/KT_Door_Close_Cue.KT_Door_Close_Cue" (Transformation|GetActorLocation) "0, 0, 0" 1.0 1.0 0.0 0 0 0 0)
  (Components|Timeline|SetPlayRate (Variables|Default|GetRotationTimeline) (/ 1.0 (Variables|Default|GetCloseDuration)))
  (bind _rotationcurve (Timeline|RotationTimeline Play)
    (:Update
      (Transformation|SetActorRotation (Math|Rotator|MakeRotator (.roll _startrotation) (.pitch _startrotation) (Math|Float|Lerp (.yaw _startrotation) (Variables|Default|GetClosedRotationZ) _rotationcurve))))))

(event EventBeginPlay
  (Variables|Default|SetStartRotation (Transformation|GetActorRotation)))

(fn ConstructionScript)