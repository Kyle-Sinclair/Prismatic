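; BP_KillTunnelWall is a moving wall in the KillTunnel trap that slides from its starting spot to the owning KillTunnel's location.
; MoveWall runs a timeline scaled by TrapDuration, lerping position without sweep, then stops its Niagara effect and has the KillTunnel play crash FX.
; Separate events start the wake-up and movement effects or reset both.
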(event Custom|MoveWall
  (Components|Timeline|SetPlayRate (Variables|Default|GetTimeline) (/ 1.0 (Variables|Default|GetTrapDuration)))
  (bind _wallmovement (Timeline|Timeline Play)
    (:Update
      (Transformation|SetActorLocation (Math|Vector|Lerp(Vector) (Variables|Default|GetStartLocation) (Transformation|GetActorLocation (Variables|Default|GetKillTunnel)) _wallmovement) false false))
    (:Finished
      (Components|Activation|Deactivate (Variables|Default|GetNiagara))
      (Default|PlayCrashFX (Variables|Default|GetKillTunnel))
      (Development|PrintString "Finished Move"))))

(event Custom|PlayWakeUpFX
  (Components|Activation|Activate (Variables|Default|GetNiagara) false))

(event Custom|PlayMoveFX
  (Components|Activation|Activate (Variables|Default|GetMoveFX) false))

(event Custom|ResetVFX
  (Components|Activation|Deactivate (Variables|Default|GetNiagara))
  (Components|Activation|Deactivate (Variables|Default|GetMoveFX)))

(event EventBeginPlay
  (Variables|Default|SetStartLocation (Transformation|GetActorLocation)))

(fn ConstructionScript)