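; Breakable rock wall that shatters, fades out and removes itself, either through its Break event or when hit by an explosion, which also plays a stone explosion sound.
; Breaking runs once, enabling physics on the Geometry Collection and removing the cube and box components.
; A timeline then drives the "Trans" parameter on dynamic instances of the collection's three materials to fade the debris before destroying the actor.
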(event Custom|Break
  ;[1 1 1] Breaking rock
  (Utilities|FlowControl|DoOnce false
    (:Completed
      (Physics|SetSimulatePhysics (Variables|Default|GetGeometryCollection) true)
      (CallFunction|Destroy))))

(event Custom|Destroy
  ;[1 1 1] Destroy + fade
  (Components|DestroyComponent (Variables|Default|GetCube1))
  (Components|DestroyComponent (Variables|Default|GetCube2))
  (Components|DestroyComponent (Variables|Default|GetCube3))
  (Components|DestroyComponent (Variables|Default|GetBox))
  (bind _returnvalue (Rendering|Material|CreateDynamicMaterialInstance (Variables|Default|GetGeometryCollection) 0 "/Game/Art/Material/Material_instances/MI_BreakWall.MI_BreakWall" "None" :!class /Script/Engine.PrimitiveComponent))
  (bind _returnvalue_2 (Rendering|Material|CreateDynamicMaterialInstance (Variables|Default|GetGeometryCollection) 1 "/Game/Art/Material/Material_instances/MI_tiling_rock_2_Inst_2.MI_tiling_rock_2_Inst_2" "None" :!class /Script/Engine.PrimitiveComponent))
  (bind _returnvalue_3 (Rendering|Material|CreateDynamicMaterialInstance (Variables|Default|GetGeometryCollection) 2 "/Game/Art/Material/Material_instances/MI_tiling_rock_2_Inst_2.MI_tiling_rock_2_Inst_2" "None" :!class /Script/Engine.PrimitiveComponent))
  (bind _output_get (Variables|Default|SetMaterial (Utilities|Array|MakeArray _returnvalue _returnvalue_2 _returnvalue_3)))
  (bind _newtrack_0 (Timeline|Timeline Play)
    (:Update
      (for _array_element _output_get
        (Rendering|Material|SetScalarParameterValue _array_element "Trans" _newtrack_0 :!class /Script/Engine.MaterialInstanceDynamic)))
    (:Finished
      (Actor|DestroyActor))))

(event EventOnHitbyExplosion
  (params (Satchel :type Actor%20Object%20Reference))
  ;[1 1 1] Break rock with explosion
  (Utilities|FlowControl|DoOnce false
    (:Completed
      (CallFunction|Break)
      (Audio|PlaySoundatLocation "/Game/Audio/Level/Stones/Stone_Explode__Cue.Stone_Explode__Cue" (Transformation|GetActorLocation) "0, 0, 0" 1.0 1.0 0.0 0 0 0 0))))

(fn ConstructionScript)