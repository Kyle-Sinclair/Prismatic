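; BP_Breakable_KillTunnel is a breakable rock that shatters, typically when hit by an explosion.
; Break enables physics on its geometry collection, removes its box collision, then destroys the actor after a short delay.
; An explosion hit notifies the owning BP_Spawner through OnDestroy, then triggers Break and plays a stone explosion sound; it does nothing without a spawner owner.
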(event Custom|Break
  ;[1 1 1] Breaking rock
  (Physics|SetSimulatePhysics (Variables|Default|GetGeometryCollection) true)
  (Components|DestroyComponent (Variables|Default|GetBox))
  (Utilities|FlowControl|Delay 0.5)
  (Actor|DestroyActor))

(event EventOnHitbyExplosion
  (params (Satchel :type Actor%20Object%20Reference))
  ;[1 1 1] Break rock with explosion
  (bind _asbp_spawner (Utilities|Casting|CastToBP_Spawner (Components|GetOwner)))
  (Default|OnDestroy _asbp_spawner)
  (CallFunction|Break)
  (Audio|PlaySoundatLocation "/Game/Audio/Level/Stones/Stone_Explode__Cue.Stone_Explode__Cue" (Transformation|GetActorLocation) "0, 0, 0" 1.0 1.0 0.0 0 0 0 0))

(fn ConstructionScript)