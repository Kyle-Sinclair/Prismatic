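; Temporary level trigger actor that grants a configured ability to a ProtoMovementCharacter entering its TriggerArea.
; On overlap it acts only if the character lacks that ability, calling GiveAbility for regular abilities.
; The dash charges ability is a special case: it sets the character's dash charges to ChargeAmount when their maximum is lower, without calling GiveAbility.
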(event OnComponentBeginOverlap(TriggerArea)
  (params (OverlappedComponent :type Primitive%20Component%20Object%20Reference) (OtherActor :type Actor%20Object%20Reference) (OtherComp :type Primitive%20Component%20Object%20Reference) (OtherBodyIndex :type Integer) (bFromSweep :type Boolean) (SweepResult :type Hit%20Result%20Structure%20%28by%20ref%29))
  (bind _ability (Variables|Default|GetAbility))
  (bind _chargeamount (Variables|Default|GetChargeAmount))
  (bind _asproto_movement_character (Utilities|Casting|CastToProtoMovementCharacter OtherActor))
  (bind _returnvalue (Class|ProtoMovementCharacter|HasAbility _asproto_movement_character _ability))
  (if (not _returnvalue)
    (if (Utilities|Enum|Equal(Enum) _ability "Ability_DashCharges")
      (if (< (Class|ProtoMovementCharacter|GetMaxDashCharges _asproto_movement_character) _chargeamount)
        (Class|ProtoMovementCharacter|SetDashCharges _asproto_movement_character _chargeamount))
      (else
        (Class|ProtoMovementCharacter|GiveAbility _asproto_movement_character _ability)))))

(fn ConstructionScript)