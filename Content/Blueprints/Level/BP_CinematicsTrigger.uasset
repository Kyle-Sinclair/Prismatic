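; BP_CinematicsTrigger is a level trigger that plays a chosen level sequence when the player walks into it.
; On BeginPlay it gets the cinematics manager from BP_GP3GameMode and caches it, printing an error if either cast fails.
; On overlap by player 0's character, it passes LevelSequenceToPlay to the manager's PlayCinematic, then destroys itself, so it fires only once.
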(event EventBeginPlay
  ;[1 1 1] Get Reference To the cinematics System
  (bind _asbp_gp3game_mode (Utilities|Casting|CastToBP_GP3GameMode (Game|GetGameMode))
    (:then
      (bind _asbp_cinematics_manager (Utilities|Casting|CastToBP_CinematicsManager (Class|GP3GameMode|GetCinematicManager _asbp_gp3game_mode))
        (:then
          (Variables|Default|SetBP_CinematicsManagerRef _asbp_cinematics_manager))
        (:CastFailed
          (Development|PrintString "Cannot cast cinematics manager to the correct BP"))))
    (:CastFailed
      (Development|PrintString "Cannot cast game mode to the correct BP"))))

(event Collision|EventActorBeginOverlap
  (params (OtherActor :type Actor%20Object%20Reference))
  ;[1 1 1] Call Manager in response to player character
  (Utilities|Casting|CastToCharacter OtherActor)
  (if (== OtherActor (Game|GetPlayerCharacter 0))
    (Default|PlayCinematic (Variables|Default|GetBP_CinematicsManagerRef) (Variables|Default|GetLevelSequenceToPlay))
    (Actor|DestroyActor)))

(fn ConstructionScript)