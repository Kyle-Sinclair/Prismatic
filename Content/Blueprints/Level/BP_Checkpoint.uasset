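; Checkpoint actor that becomes the active respawn point when a Character overlaps its capsule.
; Begin or end overlap fires a DoOnce that registers it with the resurrection manager from the game mode and saves a height-adjusted location through the game instance.
; Activation swaps the Niagara effect, plays a sound and shows a widget that timers fade out and remove.
; ResetCheckpoint restores the inactive effect and re-arms the DoOnce.
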(event OnComponentBeginOverlap(Capsule)
  (params (OverlappedComponent :type Primitive%20Component%20Object%20Reference) (OtherActor :type Actor%20Object%20Reference) (OtherComp :type Primitive%20Component%20Object%20Reference) (OtherBodyIndex :type Integer) (bFromSweep :type Boolean) (SweepResult :type Hit%20Result%20Structure%20%28by%20ref%29))
  ;[1 1 1] Check if Player
  (bind _ascharacter (Utilities|Casting|CastToCharacter OtherActor))
  (Variables|Default|SetCharacter _ascharacter)
  (Utilities|IsValid (Variables|Default|GetBP%20ResManager)
    (:Is%20Valid
      (Utilities|FlowControl|DoOnce false
        (:Completed
          ;[1 1 1] Update Res Manager's current check point
          (Default|ChangeCheckpoint (Variables|Default|GetBP%20ResManager) self)
          (bind _asbp_gp3game_instance (Utilities|Casting|CastToBP_GP3GameInstance (Game|GetGameInstance)))
          (Class|GP3GameInstance|WriteCheckPointtoCurrentSaveFile _asbp_gp3game_instance (+ (Transformation|GetActorLocation) (* (Components|Capsule|GetScaledCapsuleHalfHeight (Variables|/Script/Engine.Character|GetCapsuleComponent (Variables|Default|GetCharacter))) (Math|Vector|VectorUp))))
          (Class|GP3GameInstance|SaveCurrentSaveFiletoSlot _asbp_gp3game_instance)
          ;[1 1 1] Setting activation vfx and sfx
          (Class|NiagaraComponent|SetAsset (Variables|Default|GetNiagara) "/Game/Art/VFX/FXS_REspawnpoint_Active.FXS_REspawnpoint_Active" true)
          (Audio|PlaySoundatLocation "/Game/Audio/Level/Environment/Dynamic_Ambiences/Checkpoint_Activated_Cue.Checkpoint_Activated_Cue" (Transformation|GetWorldLocation (Variables|Default|GetCapsule)) "0, 0, 0" 1.0 1.0 0.0 0 0 0 0)
          (bind _returnvalue (UserInterface|CreateWidget "/Game/Blueprints/Widget/WBP_CheckpointActivated.WBP_CheckpointActivated_C"))
          (bind _output_get (Variables|Default|SetWdigetActivated _returnvalue))
          (UserInterface|Viewport|AddtoViewport _output_get 0)
          (Utilities|Time|SetTimerbyEvent (delegate Custom|FadeOutWidget) 1.2))))))

(event OnComponentEndOverlap(Capsule)
  (params (OverlappedComponent :type Primitive%20Component%20Object%20Reference) (OtherActor :type Actor%20Object%20Reference) (OtherComp :type Primitive%20Component%20Object%20Reference) (OtherBodyIndex :type Integer))
  ;[1 1 1] Check if Player
  (bind _ascharacter (Utilities|Casting|CastToCharacter OtherActor))
  (Variables|Default|SetCharacter _ascharacter)
  (Utilities|IsValid (Variables|Default|GetBP%20ResManager)
    (:Is%20Valid
      (Utilities|FlowControl|DoOnce false
        (:Completed
          ;[1 1 1] Update Res Manager's current check point
          (Default|ChangeCheckpoint (Variables|Default|GetBP%20ResManager) self)
          (bind _asbp_gp3game_instance (Utilities|Casting|CastToBP_GP3GameInstance (Game|GetGameInstance)))
          (Class|GP3GameInstance|WriteCheckPointtoCurrentSaveFile _asbp_gp3game_instance (+ (Transformation|GetActorLocation) (* (Components|Capsule|GetScaledCapsuleHalfHeight (Variables|/Script/Engine.Character|GetCapsuleComponent (Variables|Default|GetCharacter))) (Math|Vector|VectorUp))))
          (Class|GP3GameInstance|SaveCurrentSaveFiletoSlot _asbp_gp3game_instance)
          ;[1 1 1] Setting activation vfx and sfx
          (Class|NiagaraComponent|SetAsset (Variables|Default|GetNiagara) "/Game/Art/VFX/FXS_REspawnpoint_Active.FXS_REspawnpoint_Active" true)
          (Audio|PlaySoundatLocation "/Game/Audio/Level/Environment/Dynamic_Ambiences/Checkpoint_Activated_Cue.Checkpoint_Activated_Cue" (Transformation|GetWorldLocation (Variables|Default|GetCapsule)) "0, 0, 0" 1.0 1.0 0.0 0 0 0 0)
          (bind _returnvalue (UserInterface|CreateWidget "/Game/Blueprints/Widget/WBP_CheckpointActivated.WBP_CheckpointActivated_C"))
          (bind _output_get (Variables|Default|SetWdigetActivated _returnvalue))
          (UserInterface|Viewport|AddtoViewport _output_get 0)
          (Utilities|Time|SetTimerbyEvent (delegate Custom|FadeOutWidget) 1.2))))))

(event Custom|Reset%20Checkpoint
  (Class|NiagaraComponent|SetAsset (Variables|Default|GetNiagara) "/Game/Art/VFX/FXS_REspawnpoint.FXS_REspawnpoint" true)
  (Utilities|FlowControl|DoOnce false) ; enters at Reset
)

(event Custom|FadeOutWidget
  ;[1 1 1] Setting activation vfx and sfx
  (Default|PlayFadeOut (Variables|Default|GetWdigetActivated))
  (bind _returnvalue (Utilities|Time|SetTimerbyEvent (delegate Custom|RemoveWidget) 0.1 true)))

(event Custom|RemoveWidget
  (bind _wdigetactivated (Variables|Default|GetWdigetActivated))
  ;[1 1 1] Setting activation vfx and sfx
  (if (not (Class|UserWidget|IsAnimationPlaying _wdigetactivated (Variables|/Game/Blueprints/Widget/WBP_CheckpointActivated.WBP_CheckpointActivated_C|GetFadeOut _wdigetactivated)))
    (Widget|RemovefromParent (Variables|Default|GetWdigetActivated))
    (Utilities|Time|ClearandInvalidateTimerbyHandle (stale Custom|FadeOutWidget _returnvalue))))

(event EventBeginPlay
  (Utilities|FlowControl|Sequence
    (:then_0
      ;[1 1 1] Get Reference To Res System
      (bind _asbp_gp3game_mode (Utilities|Casting|CastToBP_GP3GameMode (Game|GetGameMode)))
      (bind _asbp_resurrection_manager (Utilities|Casting|CastToBP_ResurrectionManager (Class|GP3GameMode|GetResManager _asbp_gp3game_mode))
        (:then
          (Variables|Default|SetBP%20ResManager _asbp_resurrection_manager))
        (:CastFailed
          (Development|PrintString "A checkpoint failed to get a reference to the resurrection system"))))))

(fn ConstructionScript)