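; BP_TutorialSign is a level tutorial sign whose prompt widget rotates to face the camera and appears when a Character enters its trigger.
; OnInteract toggles a WBP_TutorialPrompt viewport widget that plays the configured media, hiding the world prompt and blocking move and look input while open.
; A DoOnce reset by a short timer debounces interaction.
; Leaving the trigger hides the prompt, removes the video and restores input.
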(event OnComponentBeginOverlap(Trigger_TutorialPrompt)
  (params (OverlappedComponent :type Primitive%20Component%20Object%20Reference) (OtherActor :type Actor%20Object%20Reference) (OtherComp :type Primitive%20Component%20Object%20Reference) (OtherBodyIndex :type Integer) (bFromSweep :type Boolean) (SweepResult :type Hit%20Result%20Structure%20%28by%20ref%29))
  (Utilities|Casting|CastToCharacter OtherActor)
  (Rendering|SetVisibility (Variables|Default|GetWidget) true false))

(event OnComponentEndOverlap(Trigger_TutorialPrompt)
  (params (OverlappedComponent :type Primitive%20Component%20Object%20Reference) (OtherActor :type Actor%20Object%20Reference) (OtherComp :type Primitive%20Component%20Object%20Reference) (OtherBodyIndex :type Integer))
  (bind _returnvalue (Game|GetPlayerController 0))
  (Utilities|Casting|CastToCharacter OtherActor)
  (Rendering|SetVisibility (Variables|Default|GetWidget) false false)
  (Variables|Default|SetInteractSwitch 0)
  (bind _tutorialwidget (Variables|Default|GetTutorialWidget)
    (:then
      (Widget|RemovefromParent _tutorialwidget)
      (Utilities|IsValid _returnvalue
        (:Is%20Valid
          (Input|ResetIgnoreMoveInput _returnvalue)
          (Input|ResetIgnoreLookInput _returnvalue))
        (:Is%20Not%20Valid
          (Development|PrintString "no controller"))))
    (:else)))

(event Custom|PlayTutorialVideo
  ;[1 1 1] Comment
  (bind _returnvalue (UserInterface|CreateWidget "/Game/Blueprints/Widget/TutorialPrompt/WBP_TutorialPrompt.WBP_TutorialPrompt_C"))
  (bind _output_get (Variables|Default|SetTutorialWidget _returnvalue))
  (UserInterface|Viewport|AddtoViewport _output_get 0)
  (Default|SetDisplayPrompt _output_get (Variables|Default|GetNew%20Media%20Source) (Variables|Default|GetNew%20Prompt%20Background))
  (Default|PlayMedia _output_get)
  (Rendering|SetVisibility (Variables|Default|GetWidget) false false))

(event Custom|RemoveTutorialVideo
  (bind _tutorialwidget (Variables|Default|GetTutorialWidget)
    (:then
      (Widget|RemovefromParent _tutorialwidget)
      (Rendering|SetVisibility (Variables|Default|GetWidget) true false))
    (:else)))

(event Custom|ResetInteract
  (bind _returnvalue (Game|GetPlayerController 0))
  (bind _returnvalue_2 (Game|GetPlayerController 0))
  (Utilities|FlowControl|DoOnce false) ; enters at Reset
)

(event EventTick
  (params (DeltaSeconds :type Float%20%28single-precision%29))
  (Transformation|SetWorldRotation (Variables|Default|GetWidget) (Math|Rotator|FindLookatRotation (Transformation|GetWorldLocation (Variables|Default|GetWidget)) (Transformation|GetActorLocation (Game|GetPlayerCameraManager 0))) false false))

(event EventBeginPlay
  (Variables|Default|SetPlayerRef (Pawn|GetControlledPawn (Game|GetPlayerController 0)))
  (Rendering|SetCastShadow (Variables|Default|GetWidget) false))

(event EventOnInteract
  (bind _returnvalue (Game|GetPlayerController 0))
  (bind _returnvalue_2 (Game|GetPlayerController 0))
  (Utilities|FlowControl|DoOnce false
    (:Completed
      (switch int (Variables|Default|GetInteractSwitch)
        (:0
          (CallFunction|PlayTutorialVideo)
          (Input|SetIgnoreMoveInput _returnvalue true)
          (Input|SetIgnoreLookInput _returnvalue true)
          (Variables|Default|SetInteractSwitch 1))
        (:1
          (CallFunction|RemoveTutorialVideo)
          (Input|SetIgnoreMoveInput _returnvalue_2 false)
          (Input|SetIgnoreLookInput _returnvalue_2 false)
          (Variables|Default|SetInteractSwitch 0)))
      (bind _returnvalue_3 (Utilities|Time|SetTimerbyEvent (delegate Custom|ResetInteract) 0.4))
      (Variables|Default|SetTimer_Reset _returnvalue_3))))

(fn ConstructionScript)