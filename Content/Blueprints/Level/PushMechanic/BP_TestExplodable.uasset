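; BP_TestExplodable is a test explodable for the push mechanic that moves another object when a satchel explosion hits it at close range.
; OnHitbyExplosion measures the distance to the Satchel and, under a fixed threshold, calls Move on AffectedObject with MoveDirection.
; Hits at or beyond that threshold only print the measured distance as debug output.
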(event EventOnHitbyExplosion
  (params (Satchel :type Actor%20Object%20Reference))
  (bind _returnvalue (Transformation|GetActorLocation Satchel))
  (bind _returnvalue_2 (Transformation|GetActorLocation))
  (bind _returnvalue_3 (- _returnvalue _returnvalue_2))
  (bind _returnvalue_4 (Math|Vector|VectorLength _returnvalue_3))
  (if (< _returnvalue_4 1e+02)
    (Default|Move (Variables|Default|GetAffectedObject) (Variables|Default|GetMoveDirection))
    (else
      (Development|PrintString (Utilities|String|ToString(Float) _returnvalue_4)))))

(fn ConstructionScript)