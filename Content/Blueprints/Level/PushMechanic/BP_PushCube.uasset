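; Pushable cube that bomb explosions move one point at a time along a referenced spline.
; A blast within range and roughly aligned with a forward or backward explodable component picks the direction, using an offset dot-product test.
; A timeline eases the actor to the next spline point with a drag sound.
; While moving, side boxes knock characters away; a failsafe box stops and teleports overlapping characters aside.
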(event OnComponentBeginOverlap(Box)
  (params (OverlappedComponent :type Primitive%20Component%20Object%20Reference) (OtherActor :type Actor%20Object%20Reference) (OtherComp :type Primitive%20Component%20Object%20Reference) (OtherBodyIndex :type Integer) (bFromSweep :type Boolean) (SweepResult :type Hit%20Result%20Structure%20%28by%20ref%29))
  (Utilities|KnockbackMacro OtherActor (Variables|Default|GetCurrentDirection)))

(event OnComponentBeginOverlap(Box1)
  (params (OverlappedComponent :type Primitive%20Component%20Object%20Reference) (OtherActor :type Actor%20Object%20Reference) (OtherComp :type Primitive%20Component%20Object%20Reference) (OtherBodyIndex :type Integer) (bFromSweep :type Boolean) (SweepResult :type Hit%20Result%20Structure%20%28by%20ref%29))
  (Utilities|KnockbackMacro OtherActor (Variables|Default|GetCurrentDirection)))

(event OnComponentBeginOverlap(FailSafe)
  (params (OverlappedComponent :type Primitive%20Component%20Object%20Reference) (OtherActor :type Actor%20Object%20Reference) (OtherComp :type Primitive%20Component%20Object%20Reference) (OtherBodyIndex :type Integer) (bFromSweep :type Boolean) (SweepResult :type Hit%20Result%20Structure%20%28by%20ref%29))
  (bind _ascharacter (Utilities|Casting|CastToCharacter OtherActor))
  (Variables|/Script/Engine.MovementComponent|SetVelocity (Variables|/Script/Engine.Character|GetCharacterMovement _ascharacter) "0, 0, 0")
  (Transformation|SetActorLocation _ascharacter (+ (Transformation|GetActorLocation) (Math|Vector|MakeVector 0.0 2e+02 0.0)) false true))

(event Custom|Move
  (params (Direction :type Integer))
  (if (not (Variables|Default|GetIsMoving))
    (if (== Direction 1)
      (Variables|Default|SetCurrentDirection 1.0)
      (if (< (Variables|Default|GetCurrentSplineIndex) (- (Spline|GetNumberOfSplinePoints (Variables|/Game/Blueprints/Level/PushMechanic/BP_PushSpline.BP_PushSpline_C|GetSpline (Variables|Default|GetPushSpline))) 1))
        (Math|Integer|IncrementInt (Variables|Default|GetCurrentSplineIndex)
          (:%20%20
            (Audio|PlaySoundatLocation "/Game/Audio/Level/Stones/Stone_Drag_Small__Cue.Stone_Drag_Small__Cue" (Transformation|GetWorldLocation (Variables|Default|GetCube)) "0, 0, 0" 1.0 1.0 0.0 0 0 0 0 :!label _label)
            (Components|Timeline|SetPlayRate (Variables|Default|GetPushTimeline) (/ 1.0 (Variables|Default|GetPushDuration)))
            (Variables|Default|SetIsMoving true)
            (bind _forcecurve (Timeline|PushTimeline PlayFromStart)
              (:Update
                (Transformation|SetActorTransform (Math|Transform|Lerp(Transform) (Transformation|GetActorTransform) (Spline|GetTransformatSplinePoint (Variables|/Game/Blueprints/Level/PushMechanic/BP_PushSpline.BP_PushSpline_C|GetSpline (Variables|Default|GetPushSpline)) (Variables|Default|GetCurrentSplineIndex) "World" false) _forcecurve)))
              (:Finished
                (Variables|Default|SetIsMoving false))))))
      (elif (== Direction -1)
        (Variables|Default|SetCurrentDirection -1.0)
        (if (> (Variables|Default|GetCurrentSplineIndex) 0)
          (Math|Integer|DecrementInt (Variables|Default|GetCurrentSplineIndex)
            (:%20%20
              (goto _label))))))))

(event EventBeginPlay
  (Transformation|SetActorTransform (Spline|GetTransformatSplinePoint (Variables|/Game/Blueprints/Level/PushMechanic/BP_PushSpline.BP_PushSpline_C|GetSpline (Variables|Default|GetPushSpline)) (Variables|Default|GetCurrentSplineIndex) "World" false)))

(event EventDoSpecificThing
  (params (TriggeringBomb :type Bomb%20Actor%20Object%20Reference) (TriggeringExplodableComponent :type Mesh%20Explodable%20Component%20Object%20Reference))
  (bind _returnvalue (Transformation|GetActorLocation TriggeringBomb))
  (bind _returnvalue_2 (Transformation|GetWorldLocation TriggeringExplodableComponent))
  (bind _cube (Variables|Default|GetCube))
  (bind _distanceforwardoffset (Variables|Default|GetDistanceForwardOffset))
  (bind _returnvalue_3 (Transformation|GetWorldLocation _cube))
  (bind _returnvalue_4 (- _returnvalue_2 _returnvalue))
  (bind _returnvalue_5 (- _returnvalue_3 _returnvalue_2))
  (bind _returnvalue_6 (Math|Vector|Normalize _returnvalue_5))
  (bind _returnvalue_7 (* _returnvalue_6 _distanceforwardoffset))
  (bind _returnvalue_8 (+ _returnvalue_7 _returnvalue_4))
  (bind _returnvalue_9 (Math|Vector|Normalize _returnvalue_8))
  (bind _returnvalue_10 (Math|Vector|DotProduct _returnvalue_6 _returnvalue_9))
  (bind _returnvalue_11 (Math|Float|Sign(Float) _returnvalue_10))
  (bind _returnvalue_12 (* _returnvalue_10 _returnvalue_10))
  (bind _returnvalue_13 (* _returnvalue_11 _returnvalue_12))
  (if (Utilities|IsValid TriggeringBomb)
    (Development|PrintString (Utilities|String|ToString(Float) _returnvalue_13))
    (if (and (> _returnvalue_13 0.0) (< (Math|Vector|VectorLength _returnvalue_4) (Variables|Default|GetPush%20Radius)))
      (CallFunction|Move (Math|Integer|SelectInt 1 -1 (== TriggeringExplodableComponent (Variables|Default|GetMeshExplodable_Forward)))))))

(fn ConstructionScript)