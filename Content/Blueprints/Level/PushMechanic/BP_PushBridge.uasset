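; Bridge that bomb blasts push one point at a time along a spline, starting at its current index.
; A blast within range and roughly aligned toward the center moves it forward or back, depending on which explodable mesh was hit.
; A timeline lerps the actor from its current transform to the target point with sweep and a drag sound.
; While moving, its overlap boxes launch characters, using forward-vector X for both horizontal axes.
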(event OnComponentBeginOverlap(BoxBackPlate1)
  (params (OverlappedComponent :type Primitive%20Component%20Object%20Reference) (OtherActor :type Actor%20Object%20Reference) (OtherComp :type Primitive%20Component%20Object%20Reference) (OtherBodyIndex :type Integer) (bFromSweep :type Boolean) (SweepResult :type Hit%20Result%20Structure%20%28by%20ref%29))
  (Utilities|KnockbackMacro OtherActor (Variables|Default|GetCurrentDirection)))

(event OnComponentBeginOverlap(BoxBackLegR)
  (params (OverlappedComponent :type Primitive%20Component%20Object%20Reference) (OtherActor :type Actor%20Object%20Reference) (OtherComp :type Primitive%20Component%20Object%20Reference) (OtherBodyIndex :type Integer) (bFromSweep :type Boolean) (SweepResult :type Hit%20Result%20Structure%20%28by%20ref%29))
  (Utilities|KnockbackMacro OtherActor (Variables|Default|GetCurrentDirection)))

(event OnComponentBeginOverlap(BoxBackLegL)
  (params (OverlappedComponent :type Primitive%20Component%20Object%20Reference) (OtherActor :type Actor%20Object%20Reference) (OtherComp :type Primitive%20Component%20Object%20Reference) (OtherBodyIndex :type Integer) (bFromSweep :type Boolean) (SweepResult :type Hit%20Result%20Structure%20%28by%20ref%29))
  (Utilities|KnockbackMacro OtherActor (Variables|Default|GetCurrentDirection)))

(event OnComponentBeginOverlap(BoxBackPlate)
  (params (OverlappedComponent :type Primitive%20Component%20Object%20Reference) (OtherActor :type Actor%20Object%20Reference) (OtherComp :type Primitive%20Component%20Object%20Reference) (OtherBodyIndex :type Integer) (bFromSweep :type Boolean) (SweepResult :type Hit%20Result%20Structure%20%28by%20ref%29))
  (Utilities|KnockbackMacro OtherActor (Variables|Default|GetCurrentDirection)))

(event OnComponentBeginOverlap(BoxBackLegL1)
  (params (OverlappedComponent :type Primitive%20Component%20Object%20Reference) (OtherActor :type Actor%20Object%20Reference) (OtherComp :type Primitive%20Component%20Object%20Reference) (OtherBodyIndex :type Integer) (bFromSweep :type Boolean) (SweepResult :type Hit%20Result%20Structure%20%28by%20ref%29))
  (Utilities|KnockbackMacro OtherActor (Variables|Default|GetCurrentDirection)))

(event OnComponentBeginOverlap(BoxBackLegR1)
  (params (OverlappedComponent :type Primitive%20Component%20Object%20Reference) (OtherActor :type Actor%20Object%20Reference) (OtherComp :type Primitive%20Component%20Object%20Reference) (OtherBodyIndex :type Integer) (bFromSweep :type Boolean) (SweepResult :type Hit%20Result%20Structure%20%28by%20ref%29))
  (Utilities|KnockbackMacro OtherActor (Variables|Default|GetCurrentDirection)))

(event Custom|Move
  (params (Direction :type Integer64))
  (if (not (Variables|Default|GetbIsMoving))
    (if (== Direction 1)
      (Variables|Default|SetCurrentDirection 1.0)
      (if (< (Variables|Default|GetCurrentSplineIndex) (- (Spline|GetNumberOfSplinePoints (Variables|/Game/Blueprints/Level/PushMechanic/BP_PushSpline.BP_PushSpline_C|GetSpline (Variables|Default|GetPushSpline))) 1))
        (Development|PrintString "Forward")
        (Math|Integer|IncrementInt (Variables|Default|GetCurrentSplineIndex)
          (:%20%20
            (Audio|PlaySoundatLocation "/Game/Audio/Level/Stones/Stone_Wheel_Bridge_Drag__Cue.Stone_Wheel_Bridge_Drag__Cue" (Transformation|GetWorldLocation (Variables|Default|GetObjectMesh)) "0, 0, 0" 1.0 1.0 0.0 0 0 0 0 :!label _label)
            (Components|Timeline|SetPlayRate (Variables|Default|GetPushTimeline) (/ 1.0 (Variables|Default|GetPushDuration)))
            (Variables|Default|SetbIsMoving true)
            (bind _forcecurve (Timeline|PushTimeline PlayFromStart)
              (:Update
                (Transformation|SetActorTransform (Math|Transform|Lerp(Transform) (Transformation|GetActorTransform) (Spline|GetTransformatSplinePoint (Variables|/Game/Blueprints/Level/PushMechanic/BP_PushSpline.BP_PushSpline_C|GetSpline (Variables|Default|GetPushSpline)) (Variables|Default|GetCurrentSplineIndex) "World" false) _forcecurve) true))
              (:Finished
                (Variables|Default|SetbIsMoving false)
                (Development|PrintString "done"))))))
      (elif (== Direction -1)
        (Variables|Default|SetCurrentDirection -1.0)
        (if (> (Variables|Default|GetCurrentSplineIndex) 0)
          (Development|PrintString "Reverse")
          (Math|Integer|DecrementInt (Variables|Default|GetCurrentSplineIndex)
            (:%20%20
              (goto _label))))))))

(event EventBeginPlay
  (Transformation|SetActorTransform (Spline|GetTransformatSplinePoint (Variables|/Game/Blueprints/Level/PushMechanic/BP_PushSpline.BP_PushSpline_C|GetSpline (Variables|Default|GetPushSpline)) (Variables|Default|GetCurrentSplineIndex) "World" false)))

(event EventDoSpecificThing
  (params (TriggeringBomb :type Bomb%20Actor%20Object%20Reference) (TriggeringExplodableComponent :type Mesh%20Explodable%20Component%20Object%20Reference))
  (bind _returnvalue (Transformation|GetActorLocation TriggeringBomb))
  (bind _returnvalue_2 (Transformation|GetWorldLocation TriggeringExplodableComponent))
  (bind _center (Variables|Default|GetCenter))
  (bind _distanceforwardoffset (Variables|Default|GetDistanceForwardOffset))
  (bind _returnvalue_3 (Transformation|GetWorldLocation _center))
  (bind _returnvalue_4 (- _returnvalue_2 _returnvalue))
  (bind _returnvalue_5 (- _returnvalue_3 _returnvalue_2))
  (bind _returnvalue_6 (Math|Vector|Normalize _returnvalue_5))
  (bind _returnvalue_7 (* _returnvalue_6 _distanceforwardoffset))
  (bind _returnvalue_8 (+ _returnvalue_7 _returnvalue_4))
  (bind _returnvalue_9 (Math|Vector|Normalize _returnvalue_8))
  (bind _returnvalue_10 (Math|Vector|DotProduct _returnvalue_6 _returnvalue_9))
  (Utilities|IsValid TriggeringBomb
    (:Is%20Valid
      (if (and (> (* (Math|Float|Sign(Float) _returnvalue_10) (* _returnvalue_10 _returnvalue_10)) 0.0) (< (Math|Vector|VectorLength _returnvalue_4) (Variables|Default|GetPushDistance)))
        (if (== TriggeringExplodableComponent (Variables|Default|GetMeshExplodable_Forward))
          (CallFunction|Move 1)
          (elif (== TriggeringExplodableComponent (Variables|Default|GetMeshExplodable_Reverse))
            (CallFunction|Move -1)))))))

(fn ConstructionScript)