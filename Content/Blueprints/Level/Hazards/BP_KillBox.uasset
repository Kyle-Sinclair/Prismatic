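; BP_KillBox is a level hazard that tries to kill the player on overlap.
; On BeginPlay it caches the resurrection manager from BP_GP3GameMode, printing an error if that manager's cast fails.
; When player character 0 overlaps it, it calls TryKillPlayer on the manager and, if that succeeds, plays a falling-death sound at the character's location.
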(event Collision|EventActorBeginOverlap
  (params (OtherActor :type Actor%20Object%20Reference))
  ;[1 1 1] Call Manager in response to player character
  (bind _ascharacter (Utilities|Casting|CastToCharacter OtherActor))
  (if (== OtherActor (Game|GetPlayerCharacter 0))
    (bind _returnvalue (Class|ResurrectionManager|TryKillPlayer (Variables|Default|GetBP%20Res%20Manager)))
    (if _returnvalue
      (Audio|PlaySoundatLocation "/Game/Audio/Character/Death/Death_Fall__Cue.Death_Fall__Cue" (Transformation|GetActorLocation _ascharacter) "0, 0, 0" 1.0 1.0 0.0 0 0 0 0))))

(event EventBeginPlay
  ;[1 1 1] Get Reference To Res System
  (bind _asbp_gp3game_mode (Utilities|Casting|CastToBP_GP3GameMode (Game|GetGameMode)))
  (bind _asbp_resurrection_manager (Utilities|Casting|CastToBP_ResurrectionManager (Class|GP3GameMode|GetResManager _asbp_gp3game_mode))
    (:then
      (Variables|Default|SetBP%20Res%20Manager _asbp_resurrection_manager))
    (:CastFailed
      (Development|PrintString "A killbox failed to get a reference to the resurrection system"))))

(fn ConstructionScript)