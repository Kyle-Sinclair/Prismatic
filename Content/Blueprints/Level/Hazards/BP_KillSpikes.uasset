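; BP_KillSpikes is a level hazard that kills the player on contact.
; On BeginPlay it caches the resurrection manager from the GP3 game mode, printing an error if that cast fails.
; When a character overlaps it and is player 0's character, it calls TryKillPlayer on that manager, leaving the death handling to the resurrection system.
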(event Collision|EventActorBeginOverlap
  (params (OtherActor :type Actor%20Object%20Reference))
  (Utilities|Casting|CastToCharacter OtherActor)
  (if (== OtherActor (Game|GetPlayerCharacter 0))
    (Class|ResurrectionManager|TryKillPlayer (Variables|Default|GetBP%20Res%20Manager))))

(event EventBeginPlay
  ;[1 1 1] Get Reference To Res System
  (bind _asbp_gp3game_mode (Utilities|Casting|CastToBP_GP3GameMode (Game|GetGameMode)))
  (bind _asbp_resurrection_manager (Utilities|Casting|CastToBP_ResurrectionManager (Class|GP3GameMode|GetResManager _asbp_gp3game_mode))
    (:then
      (Variables|Default|SetBP%20Res%20Manager _asbp_resurrection_manager))
    (:CastFailed
      (Development|PrintString "A killbox failed to get a reference to the resurrection system" false))))

(fn ConstructionScript)