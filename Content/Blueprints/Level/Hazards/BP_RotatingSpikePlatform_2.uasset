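; Rotating spike platform hazard that kills the player when they touch one of its spike trigger boxes.
; On BeginPlay it caches the resurrection manager from the game mode, printing an error if that cast fails.
; Six box overlaps feed a shared KillPlayer function, which asks the manager to kill player 0 and plays a spike death sound on success.
; No rotation logic lives in these graphs.
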(event OnComponentBeginOverlap(Box6)
  (params (OverlappedComponent :type Primitive%20Component%20Object%20Reference) (OtherActor :type Actor%20Object%20Reference) (OtherComp :type Primitive%20Component%20Object%20Reference) (OtherBodyIndex :type Integer) (bFromSweep :type Boolean) (SweepResult :type Hit%20Result%20Structure%20%28by%20ref%29))
  (CallFunction|KillPlayer OtherActor))

(event OnComponentBeginOverlap(Box)
  (params (OverlappedComponent :type Primitive%20Component%20Object%20Reference) (OtherActor :type Actor%20Object%20Reference) (OtherComp :type Primitive%20Component%20Object%20Reference) (OtherBodyIndex :type Integer) (bFromSweep :type Boolean) (SweepResult :type Hit%20Result%20Structure%20%28by%20ref%29))
  (CallFunction|KillPlayer OtherActor))

(event OnComponentBeginOverlap(Box1)
  (params (OverlappedComponent :type Primitive%20Component%20Object%20Reference) (OtherActor :type Actor%20Object%20Reference) (OtherComp :type Primitive%20Component%20Object%20Reference) (OtherBodyIndex :type Integer) (bFromSweep :type Boolean) (SweepResult :type Hit%20Result%20Structure%20%28by%20ref%29))
  (CallFunction|KillPlayer OtherActor))

(event OnComponentBeginOverlap(Box2)
  (params (OverlappedComponent :type Primitive%20Component%20Object%20Reference) (OtherActor :type Actor%20Object%20Reference) (OtherComp :type Primitive%20Component%20Object%20Reference) (OtherBodyIndex :type Integer) (bFromSweep :type Boolean) (SweepResult :type Hit%20Result%20Structure%20%28by%20ref%29))
  (CallFunction|KillPlayer OtherActor))

(event OnComponentBeginOverlap(Box3)
  (params (OverlappedComponent :type Primitive%20Component%20Object%20Reference) (OtherActor :type Actor%20Object%20Reference) (OtherComp :type Primitive%20Component%20Object%20Reference) (OtherBodyIndex :type Integer) (bFromSweep :type Boolean) (SweepResult :type Hit%20Result%20Structure%20%28by%20ref%29))
  (CallFunction|KillPlayer OtherActor))

(event OnComponentBeginOverlap(Box4)
  (params (OverlappedComponent :type Primitive%20Component%20Object%20Reference) (OtherActor :type Actor%20Object%20Reference) (OtherComp :type Primitive%20Component%20Object%20Reference) (OtherBodyIndex :type Integer) (bFromSweep :type Boolean) (SweepResult :type Hit%20Result%20Structure%20%28by%20ref%29))
  (CallFunction|KillPlayer OtherActor))

(event EventBeginPlay
  ;[1 1 1] Get Reference To Res System
  (bind _asbp_gp3game_mode (Utilities|Casting|CastToBP_GP3GameMode (Game|GetGameMode)))
  (bind _asbp_resurrection_manager (Utilities|Casting|CastToBP_ResurrectionManager (Class|GP3GameMode|GetResManager _asbp_gp3game_mode))
    (:then
      (Variables|Default|SetBP_Res%20Manager _asbp_resurrection_manager))
    (:CastFailed
      (Development|PrintString "A killbox failed to get a reference to the resurrection system"))))

(fn ConstructionScript)

(fn KillPlayer
  (params (Player :type Actor%20Object%20Reference))
  (bind _ascharacter (Utilities|Casting|CastToCharacter Player))
  (if (== Player (Game|GetPlayerCharacter 0))
    (bind _returnvalue (Class|ResurrectionManager|TryKillPlayer (Variables|Default|GetBP_Res%20Manager)))
    (if _returnvalue
      (Audio|PlaySoundatLocation "/Game/Audio/Character/Death/Death_Spike_Cue.Death_Spike_Cue" (Transformation|GetActorLocation _ascharacter) "0, 0, 0" 1.0 1.0 0.0 0 0 0 0))))