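; End-of-game trigger that launches the character on a geyser and hands off to the credits and main menu.
; The first character overlap disables input, sets an upward velocity in falling mode, fires the ending geyser effect and sound, and plays a level sequence.
; Two timers then show the credits widget while unpossessing the player, and open the main menu.
; A separate TriggerGeyser event activates another Niagara effect with a supplied sound.
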(event OnComponentBeginOverlap(Trigger_End)
  (params (OverlappedComponent :type Primitive%20Component%20Object%20Reference) (OtherActor :type Actor%20Object%20Reference) (OtherComp :type Primitive%20Component%20Object%20Reference) (OtherBodyIndex :type Integer) (bFromSweep :type Boolean) (SweepResult :type Hit%20Result%20Structure%20%28by%20ref%29))
  (bind _ascharacter (Utilities|Casting|CastToCharacter OtherActor))
  (Utilities|FlowControl|DoOnce false
    (:Completed
      (Input|DisableInput _ascharacter (Game|GetPlayerController 0))
      (Variables|/Script/Engine.CharacterMovementComponent|SetGravityScale (Variables|/Script/Engine.Character|GetCharacterMovement _ascharacter) 1.75)
      (Pawn|Components|CharacterMovement|SetMovementMode (Variables|/Script/Engine.Character|GetCharacterMovement _ascharacter) "MOVE_Falling" 0)
      (Variables|/Script/Engine.MovementComponent|SetVelocity (Variables|/Script/Engine.Character|GetCharacterMovement _ascharacter) "0.000000,0.000000,3800.000000")
      (CallFunction|PlayGeyser)
      (bind _outactor (Sequencer|Player|CreateLevelSequencePlayer (Variables|Default|GetLevelSequence)))
      (Sequencer|Player|Play (Variables|/Script/LevelSequence.LevelSequenceActor|GetSequencePlayer _outactor) :!class /Script/MovieScene.MovieSceneSequencePlayer))))

(event Custom|PlayGeyser
  (CallFunction|TriggerEndGeyser)
  (Utilities|Time|SetTimerbyEvent (delegate Custom|TriggerWBP) (Variables|Default|GetTimeToCredits))
  (Utilities|Time|SetTimerbyEvent (delegate Custom|LevelTransition) (Variables|Default|GetTimeToLevelTransition)))

(event Custom|TriggerWBP
  (bind _returnvalue (Game|GetPlayerController 0))
  (bind _returnvalue_2 (UserInterface|CreateWidget "/Game/Blueprints/Level/Ending/WBP_EndCredits.WBP_EndCredits_C" _returnvalue))
  (UserInterface|Viewport|AddtoViewport _returnvalue_2 0)
  (Pawn|UnPossess _returnvalue))

(event Custom|LevelTransition
  (Game|OpenLevel(byObjectReference) "/Game/Maps/Dev/MainMenu.MainMenu"))

(event Custom|TriggerGeyser
  (params (GeyserCue :type Sound%20Cue%20Object%20Reference))
  (Components|Activation|Activate (Variables|Default|GetNiagara) true)
  (Audio|PlaySoundatLocation GeyserCue (Transformation|GetActorLocation) "0, 0, 0" 1.0 1.0 0.0 0 0 0 0))

(event Custom|TriggerEndGeyser
  (Components|Activation|Activate (Variables|Default|GetFXS_Geyser_Burst_Ending) true)
  (Audio|PlaySound2D "/Game/Audio/Level/Environment/Dynamic_Ambiences/Geysir_Explode__Cue.Geysir_Explode__Cue" 1.8 1.0 0.0 0 0 false))

(fn ConstructionScript)