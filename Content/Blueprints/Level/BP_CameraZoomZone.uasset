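; BP_CameraZoomZone is a level zone that changes the player camera's zoom while an AlchemistCharacter is inside it.
; On begin overlap it sets the character camera's zoom distance and enters zoom mode over a configurable enter time.
; On end overlap it exits zoom mode over a separate exit time, with other actors ignored by the cast.
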(event Collision|EventActorBeginOverlap
  (params (OtherActor :type Actor%20Object%20Reference))
  (bind _asalchemist_character (Utilities|Casting|CastToAlchemistCharacter OtherActor))
  (Class|ThirdPersonCamera|SetZoomDistance (Variables|/Script/GP3.AlchemistCharacter|GetCharacterCamera _asalchemist_character) (Variables|Default|GetZoom%20Distance))
  (Class|ThirdPersonCamera|EnterZoomMode (Variables|/Script/GP3.AlchemistCharacter|GetCharacterCamera _asalchemist_character) (Variables|Default|GetEnter%20Transition%20Time)))

(event Collision|EventActorEndOverlap
  (params (OtherActor :type Actor%20Object%20Reference))
  (bind _asalchemist_character (Utilities|Casting|CastToAlchemistCharacter OtherActor))
  (Class|ThirdPersonCamera|ExitZoomMode (Variables|/Script/GP3.AlchemistCharacter|GetCharacterCamera _asalchemist_character) (Variables|Default|GetExit%20Transition%20Time)))

(fn ConstructionScript)