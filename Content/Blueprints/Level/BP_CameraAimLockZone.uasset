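; BP_CameraAimLockZone is a level zone that locks the AlchemistCharacter's camera aim while the character overlaps it.
; On entry it passes RotationAim's relative rotation to CharacterCamera as the aim target and enters aim lock at EnterTransitionSpeed.
; With MirrorAimDirection on, a dot product against the aim's forward vector negates the yaw when the character enters from that forward side.
; Ending the overlap exits aim lock.
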(event Collision|EventActorBeginOverlap
  (params (OtherActor :type Actor%20Object%20Reference))
  (bind _rotationaim (Variables|Default|GetRotationAim))
  (bind _relativerotation (Variables|/Script/Engine.SceneComponent|GetRelativeRotation _rotationaim))
  (bind (_roll _pitch _yaw) (Math|Rotator|BreakRotator _relativerotation))
  (bind _asalchemist_character (Utilities|Casting|CastToAlchemistCharacter OtherActor))
  (Class|ThirdPersonCamera|SetAimTarget (Variables|/Script/GP3.AlchemistCharacter|GetCharacterCamera _asalchemist_character) (Math|Rotator|SelectRotator (Math|Rotator|SelectRotator (Math|Rotator|MakeRotator _roll _pitch (* _yaw -1.0)) _relativerotation (> (Math|Vector|DotProduct (Math|Vector|Normalize (- (Transformation|GetActorLocation OtherActor) (Transformation|GetWorldLocation _rotationaim))) (Math|Vector|GetForwardVector _relativerotation)) 0.0)) _relativerotation (Variables|Default|GetMirror%20AimDirection)))
  (Class|ThirdPersonCamera|EnterAimLock (Variables|/Script/GP3.AlchemistCharacter|GetCharacterCamera _asalchemist_character) (Variables|Default|GetEnter%20Transition%20Speed)))

(event Collision|EventActorEndOverlap
  (params (OtherActor :type Actor%20Object%20Reference))
  (bind _asalchemist_character (Utilities|Casting|CastToAlchemistCharacter OtherActor))
  (Class|ThirdPersonCamera|ExitAimLock (Variables|/Script/GP3.AlchemistCharacter|GetCharacterCamera _asalchemist_character)))

(fn ConstructionScript)