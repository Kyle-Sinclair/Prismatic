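; BP_Spawner is a level actor that spawns an instance of ObjectToSpawn at its own transform on BeginPlay.
; It keeps a reference to the latest spawn and a SpawnedCount, which spawning increments and RemoveActor or OnDestroy decrements.
; RespawnActor removes the tracked actor when the count is above zero, then spawns a new one.
; A delayed removal chain is left disconnected.
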(event Custom|SpawnActor
  ;[1 1 1] SpawnActor
  (bind _returnvalue (Game|SpawnActorfromClass (Variables|Default|GetObjectToSpawn) (Transformation|GetActorTransform) "Undefined" self 0))
  (Variables|Default|SetSpawnedActor _returnvalue)
  (Math|Integer|IncrementInt (Variables|Default|GetSpawnedCount)))

(event Custom|RemoveActor
  ;[1 1 1] RemoveActor
  (Actor|DestroyActor (Variables|Default|GetSpawnedActor))
  (Math|Integer|DecrementInt (Variables|Default|GetSpawnedCount)))

(event Custom|RespawnActor
  ;[1 1 1] RespawnActor
  (if (> (Variables|Default|GetSpawnedCount) 0)
    (CallFunction|RemoveActor)
    (CallFunction|SpawnActor)
    (else
      (CallFunction|SpawnActor))))

(event Custom|OnDestroy
  ;[1 1 1] OnDestroy
  (Math|Integer|DecrementInt (Variables|Default|GetSpawnedCount)))

(event EventBeginPlay
  (CallFunction|SpawnActor))

(fn ConstructionScript)