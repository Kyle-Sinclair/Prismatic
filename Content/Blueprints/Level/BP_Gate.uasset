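; BP_Gate is a level gate that opens once at least two geysers have been registered through AddGeiser.
; AddGeiser increments a counter and, at the threshold, waits through a delay before playing the GateDestructionSequence level sequence.
; RemoveDoor hides the gate and disables the cube's collision, with no caller in this Blueprint.
; DestroyDoor is empty, DestroyActor is unwired, and debug prints trace progress.
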(event Custom|DestroyDoor)

(event Custom|Add%20Geiser
  (Variables|Default|SetGeiserCounter (+ (Variables|Default|GetGeiserCounter) 1))
  (Development|PrintString (Utilities|String|ToString(Integer) (+ (Variables|Default|GetGeiserCounter) 1)))
  (if (>= (Variables|Default|GetGeiserCounter) 2)
    (Development|PrintString "Beginning delay")
    (Utilities|FlowControl|Delay 1e+01)
    (Development|PrintString "Calling play")
    (Sequencer|Player|Play (Variables|/Script/LevelSequence.LevelSequenceActor|GetSequencePlayer (Variables|Default|GetGateDestructionSequence)) :!class /Script/MovieScene.MovieSceneSequencePlayer)
    (else
      (Development|PrintString (Utilities|String|ToString(Integer) (Variables|Default|GetGeiserCounter))))))

(fn ConstructionScript)

(fn RemoveDoor
  (Development|PrintString "Removing door")
  (Rendering|SetVisibility (Variables|Default|GetDefaultSceneRoot) false true)
  (Collision|SetCollisionEnabled (Variables|Default|GetCube) "NoCollision"))