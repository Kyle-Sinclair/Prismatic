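; Manager that handles player death and checkpoint-based resurrection for the Alchemist character.
; It tracks the active checkpoint, resetting the previous one when a new one replaces it.
; On death it disables input and spawns WBP_DeathWidget with the checkpoint or PlayerStart location; with a checkpoint, it also realigns view and actor yaw after a short delay.
; DeathAnimationFInished restores input; the fade-panel setup is disconnected.
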(event Custom|DeathAnimationFInished
  (bind _playercharacter (Variables|Default|GetPlayerCharacter))
  (Input|EnableInput _playercharacter (Pawn|GetLocalViewingPlayerController _playercharacter))
  (Variables|Default|SetbProcessingDeath false))

(event Custom|ChangeCheckpoint
  (params (New%20Checkpoint :type BP%20Checkpoint%20Object%20Reference))
  (Utilities|IsValid (Variables|Default|GetCurrentCheckPoint)
    (:Is%20Valid
      (Default|ResetCheckpoint (Variables|Default|GetCurrentCheckPoint)))
    (:Is%20Not%20Valid
      _))
  (Variables|Default|SetCurrentCheckPoint New%20Checkpoint))

(event EventBeginPlay
  ;[1 1 1] Get Reference to character
  (bind _asalchemist_character (Utilities|Casting|CastToAlchemistCharacter (Game|GetPlayerCharacter 0)))
  (bind _output_get (Variables|Default|SetPlayerCharacter _asalchemist_character))
  (Components|Movement|StopMovementImmediately (Variables|/Script/Engine.Character|GetCharacterMovement _output_get)))

(event EventOnKillPlayer
  (bind _self self)
  (bind _playercharacter (Variables|Default|GetPlayerCharacter))
  (bind _currentcheckpoint (Variables|Default|GetCurrentCheckPoint))
  (bind _playercharacter_2 (Variables|Default|GetPlayerCharacter))
  (bind _returnvalue (Transformation|GetActorRotation _playercharacter))
  (bind _returnvalue_2 (Pawn|GetLocalViewingPlayerController _playercharacter_2))
  (bind _camera_direction (Variables|/Game/Blueprints/Level/BP_Checkpoint.BP_Checkpoint_C|GetCamera%20Direction _currentcheckpoint))
  (bind (_roll _pitch) (Math|Rotator|BreakRotator _returnvalue))
  (bind _relativerotation (Variables|/Script/Engine.SceneComponent|GetRelativeRotation _camera_direction))
  (Class|AlchemistCharacter|Die _playercharacter_2)
  (Components|Movement|StopMovementImmediately (Variables|/Script/Engine.Character|GetCharacterMovement _playercharacter_2))
  (Input|DisableInput _playercharacter_2 _returnvalue_2)
  (if (Utilities|IsValid (Variables|Default|GetCurrentCheckPoint))
    (bind _returnvalue_3 (UserInterface|CreateWidget "/Game/Blueprints/Widget/WBP_DeathWidget.WBP_DeathWidget_C" _returnvalue_2 (+ (* (Components|Capsule|GetScaledCapsuleHalfHeight (Variables|/Script/Engine.Character|GetCapsuleComponent (Variables|Default|GetPlayerCharacter))) (Math|Vector|VectorUp)) (Transformation|GetActorLocation (Variables|Default|GetCurrentCheckPoint))) _self false))
    (UserInterface|Viewport|AddtoViewport _returnvalue_3 0)
    (Utilities|FlowControl|Delay 0.4)
    (Pawn|SetControlRotation _returnvalue_2 _relativerotation)
    (Transformation|SetActorRotation _playercharacter (Math|Rotator|MakeRotator _roll _pitch (.Yaw (Math|Rotator|BreakRotator _relativerotation))))
    (else
      (bind _returnvalue_4 (UserInterface|CreateWidget "/Game/Blueprints/Widget/WBP_DeathWidget.WBP_DeathWidget_C" _returnvalue_2 (Transformation|GetActorLocation (Class|GameModeBase|FindPlayerStart (Game|GetGameMode) (Game|GetPlayerController 0))) _self false))
      (UserInterface|Viewport|AddtoViewport _returnvalue_4 0))))

(fn ConstructionScript)