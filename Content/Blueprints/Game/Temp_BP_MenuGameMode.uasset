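; Temporary menu game mode that presents the main menu and drives its camera transitions.
; OnShowMainMenu switches the view to CameraMain, plays the LS_MenuFadeIn sequence, and creates WBP_MainMenu, passing it the NewGame flag and this game mode.
; It also enables game-and-UI input with the cursor shown and New Game button focused.
; CameraLoadToSettingsMenu plays the MenuLoadIn sequence, but its view target switch has no target set.
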(event EventOnShowMainMenu
  (params (NewGame :type Boolean))
  (bind _output_get (Variables|Default|SetPlayerController (Game|GetPlayerController 0)))
  (Game|Player|SetViewTargetwithBlend _output_get (Variables|Default|GetCameraMain) 0.0 "VTBlend_Linear" 0.0 false)
  (bind _outactor (Sequencer|Player|CreateLevelSequencePlayer "/Game/LevelSequences/LS_MenuFadeIn.LS_MenuFadeIn"))
  (Sequencer|Player|Play (Variables|/Script/LevelSequence.LevelSequenceActor|GetSequencePlayer _outactor) :!class /Script/MovieScene.MovieSceneSequencePlayer)
  (bind _returnvalue (UserInterface|CreateWidget "/Game/Blueprints/Widget/WBP_MainMenu.WBP_MainMenu_C" (Variables|Default|GetPlayerController)))
  (UserInterface|Viewport|AddtoViewport _returnvalue 0)
  (Input|SetInputModeGameandUI (Variables|Default|GetPlayerController) (Variables|/Game/Blueprints/Widget/WBP_MainMenu.WBP_MainMenu_C|GetNewGameButton _returnvalue) "DoNotLock" true false)
  (Default|InitializeWidget _returnvalue NewGame self)
  (Variables|/Script/Engine.PlayerController|SetbShowMouseCursor (Variables|Default|GetPlayerController) true))

(fn ConstructionScript)

(fn CameraLoadtoSettingsMenu
  (Game|Player|SetViewTargetwithBlend (Game|GetPlayerController 0) 0 0.0 "VTBlend_Linear" 0.0 false)
  (bind _outactor (Sequencer|Player|CreateLevelSequencePlayer "/Game/LevelSequences/MenuLoadIn.MenuLoadIn"))
  (Sequencer|Player|Play (Variables|/Script/LevelSequence.LevelSequenceActor|GetSequencePlayer _outactor) :!class /Script/MovieScene.MovieSceneSequencePlayer))