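; Game instance for GP3 that tracks which dialogue trigger rows have been used and applies audio volume changes.
; Used rows are stored as bits in the DialogueTriggers integer, set by SetRowIndexUsed and tested by GetRowIndexUsed.
; Separate master, SFX and music events override their sound class volume in a sound mix, fetching custom user settings before and again after a delay.
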(event Custom|UpdateMasterVolumeSettings
  (params (NewVolume :type Float%20%28double-precision%29))
  (Class|GP3GameUserSettings|GetCustomUserSettings)
  (Audio|SetSoundMixClassOverride "/Game/Audio/SoundMix_.SoundMix_" "/Game/Audio/SFX_MasterVolume.SFX_MasterVolume" NewVolume 1.0 1.0 true)
  (Utilities|FlowControl|Delay 5.0)
  (Class|GP3GameUserSettings|GetCustomUserSettings))

(event Custom|UpdateSFXVolumeSettings
  (params (NewSFX :type Float%20%28double-precision%29))
  (Class|GP3GameUserSettings|GetCustomUserSettings)
  (Audio|SetSoundMixClassOverride "/Game/Audio/SoundMix_.SoundMix_" "/Game/Audio/SFX_EffecsVolume.SFX_EffecsVolume" NewSFX 1.0 1.0 true)
  (Utilities|FlowControl|Delay 5.0)
  (Class|GP3GameUserSettings|GetCustomUserSettings))

(event Custom|UpdateMusicVolumeSettings
  (params (NewMusic :type Float%20%28double-precision%29))
  (Class|GP3GameUserSettings|GetCustomUserSettings)
  (Audio|SetSoundMixClassOverride "/Game/Audio/SoundMix_.SoundMix_" "/Game/Audio/SFX_MusicVolume.SFX_MusicVolume" NewMusic 1.0 1.0 true)
  (Utilities|FlowControl|Delay 5.0)
  (Class|GP3GameUserSettings|GetCustomUserSettings))

(event EventSetRowIndexUsed
  (params (SetRowIndexUsed :type BP_Temp_EnumDialogue%20Enum :default "NewEnumerator0"))
  (Variables|Default|SetDialogueTriggers (Class|KismetMathLibrary|OrIntInt (Math|Float|Truncate (Math|Float|Power 2.0 (Math|Conversions|ToFloat(Byte) SetRowIndexUsed))) (Variables|Default|GetDialogueTriggers))))

(fn GetRowIndexUsed
  (params (RowIndex :type BP_Temp_EnumDialogue%20Enum :default "NewEnumerator0"))
  (bind _returnvalue (Math|Conversions|ToFloat(Byte) RowIndex))
  (bind _returnvalue_2 (Math|Float|Power 2.0 _returnvalue))
  (bind _returnvalue_3 (Math|Float|Truncate _returnvalue_2))
  (return (== _returnvalue_3 (Class|KismetMathLibrary|AndIntInt _returnvalue_3 (Variables|Default|GetDialogueTriggers)))))