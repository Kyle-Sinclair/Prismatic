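; Player camera component that drives a follow boom for the owning Character each tick.
; Auto-swivels with strong sideways input, scaled by ground speed and damped as the view tilts from level.
; Eases a distance multiplier by view pitch, growing looking down and shrinking looking up.
; Boom tracks XY directly but interpolates height, following only when grounded or after the character leaves a vertical screen safe band, until landing.
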(event EventBeginPlay
  ;[1 1 1] BeginPlay
  (bind _ascharacter (Utilities|Casting|CastToCharacter (Components|GetOwner)))
  (bind _output_get (Variables|Default|SetCharacter _ascharacter))
  (Variables|Default|SetCameraZ (.Z (Math|Vector|BreakVector (Transformation|GetActorLocation _output_get)))))

(event EventTick
  (params (DeltaSeconds :type Float%20%28single-precision%29))
  (bind _returnvalue (Math|Vector|VectorDown))
  (bind _character (Variables|Default|GetCharacter))
  (bind _returnvalue_2 (Pawn|GetControlRotation _character :!class /Script/Engine.Pawn))
  (bind _returnvalue_3 (Math|Vector|GetForwardVector _returnvalue_2))
  (bind _returnvalue_4 (Math|Vector|DotProduct _returnvalue_3 _returnvalue))
  (bind _returnvalue_5 (* _returnvalue_4 _returnvalue_4))
  (Utilities|IsValid (Variables|Default|GetCharacter)
    (:Is%20Valid
      (Utilities|FlowControl|Sequence
        (:then_0
          ;[1 1 1] Swivel Logic
          (bind _speed (CallFunction|CalcSwivelSpeed DeltaSeconds))
          (Class|ThirdPersonCamera|SwivelCamera _speed))
        (:then_1
          ;[1 1 1] Pitch Distance Adjust
          (bind _output_get (Variables|Default|SetTargetDistanceMultiplier (Math|Float|SelectFloat (Math|Interpolation|Ease "ExpoInOut" _returnvalue_5 1.0 1.2) (Math|Interpolation|Ease "CircularOut" _returnvalue_5 1.0 0.1) (> (Math|Float|Sign(Float) _returnvalue_4) 0.0))))
          (Variables|Default|SetDistanceMultiplier (Math|Interpolation|FInterpTo (Variables|Default|GetDistanceMultiplier) _output_get DeltaSeconds (Variables|BP_Variables|GetDistanceMultiplierSpeed))))
        (:then_2
          (|LocationOffset DeltaSeconds))))))

(fn SetCameraLocationOLD
  (bind _cameraboom (Variables|Default|GetCameraBoom))
  (bind _cameraz (Variables|Default|GetCameraZ))
  (bind _character (Variables|Default|GetCharacter))
  (bind _forwardoffset (LocalVariables|GetForwardOffset))
  (bind _returnvalue (Transformation|GetActorLocation _character))
  (bind _returnvalue_2 (Transformation|GetActorForwardVector _character))
  (bind _returnvalue_3 (* _forwardoffset _returnvalue_2))
  (bind _returnvalue_4 (- _returnvalue _returnvalue_3))
  (bind (_x _y) (Math|Vector|BreakVector _returnvalue_4))
  (bind _returnvalue_5 (Math|Vector|MakeVector _x _y _cameraz))
  (bind (_outhit _returnvalue_6) (Collision|SphereTraceByChannel _returnvalue_4 _returnvalue_5 (Components|Capsule|GetScaledCapsuleRadius (Variables|/Script/Engine.Character|GetCapsuleComponent _character)) "TraceTypeQuery2" false 0 "None"))
  (if _returnvalue_6
    (Transformation|SetWorldLocation _cameraboom (.Location (Collision|BreakHitResult _outhit)) false true)
    (else
      (Transformation|SetWorldLocation _cameraboom _returnvalue_5 false true))))

(fn CalcSwivelSpeed
  (params (DeltaTime :type Float%20%28double-precision%29))
  (bind _returnvalue (Math|Vector|VectorUp))
  (bind _character (Variables|Default|GetCharacter))
  (bind _returnvalue_2 (Pawn|GetControlRotation _character :!class /Script/Engine.Pawn))
  (bind _returnvalue_3 (Class|Pawn|GetLastMovementInputVector _character))
  (bind _charactermovement (Variables|/Script/Engine.Character|GetCharacterMovement _character))
  (bind _yaw (Math|Rotator|BreakRotator _returnvalue_2))
  (bind _returnvalue_4 (Math|Vector|GetUpVector _returnvalue_2))
  (bind _returnvalue_5 (Math|Vector|DotProduct _returnvalue _returnvalue_4))
  (bind _returnvalue_6 (Math|Rotator|MakeRotator 0.0 0.0 _yaw))
  (bind _returnvalue_7 (Math|Vector|GetRightVector _returnvalue_6))
  (bind _returnvalue_8 (Math|Vector|VectorGetAbs _returnvalue_7))
  (bind _returnvalue_9 (* _returnvalue_8 _returnvalue_3))
  (bind _returnvalue_10 (Math|Vector|DotProduct _returnvalue_7 _returnvalue_9))
  (return (Math|Float|SelectFloat (* (Math|Float|Power (Math|Float|Clamp(Float) (* _returnvalue_5 _returnvalue_5)) 3.0) (* (Math|Float|Sign(Float) _returnvalue_10) (* (/ (Math|Vector|VectorLengthXY (Variables|/Script/Engine.MovementComponent|GetVelocity _charactermovement)) (* 1.0 (Class|MovementComponent|GetMaxSpeed _charactermovement))) DeltaTime))) 0.0 (> (Math|Float|Absolute(Float) _returnvalue_10) 0.6))))