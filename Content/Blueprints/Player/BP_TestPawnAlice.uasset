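; BP_TestPawnAlice is a test player pawn with experimental bomb-cooldown display logic and no active event behavior.
; UpdateAbilityBar converts a cooldown into a scaled, offset "Cooldown" scalar in the MaterialDataSemtex parameter collection, so materials can reflect it.
; Its only call, fed by BPAbilityComponent's bomb cooldown alongside a debug print, is unreachable, as is an unfinished spawn-and-attach snippet.
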(event EventBeginPlay)

(event Collision|EventActorBeginOverlap
  (params (OtherActor :type Actor%20Object%20Reference)))

(event EventTick
  (params (DeltaSeconds :type Float%20%28single-precision%29)))

(fn ConstructionScript)

(fn UpdateAbilityBar
  (params (Cooldown :type Float%20%28double-precision%29))
  (bind _result (Math|Float|NegateFloat Cooldown)
    (:%20%20
      (Rendering|Material|SetScalarParameterValue "/Game/Art/UI/MaterialDataSemtex.MaterialDataSemtex" "Cooldown" (+ (/ _result 5e+01) 0.5) :!class /Script/Engine.KismetMaterialLibrary))))