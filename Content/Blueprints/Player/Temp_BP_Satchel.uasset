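; Alchemist satchel bomb that falls with extra gravity, sticks to what it hits, and asks the instigator's ability component to detonate it after a fuse.
; OnExplode launches an Alchemist in range with clear line of sight, notifies explodable actors and mesh components, then destroys itself.
; Launch force follows a distance curve, aims directly away for distant airborne players, and merges with current velocity per axis under caps for blast jumping.
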(event Collision|EventHit
  (params (MyComp :type Primitive%20Component%20Object%20Reference) (Other :type Actor%20Object%20Reference) (OtherComp :type Primitive%20Component%20Object%20Reference) (bSelfMoved :type Boolean) (HitLocation :type Vector :default "0, 0, 0") (HitNormal :type Vector :default "0, 0, 0") (NormalImpulse :type Vector :default "0, 0, 0") (Hit :type Hit%20Result%20Structure%20%28by%20ref%29))
  (bind _spherecomponent (Variables|Default|GetSphereComponent))
  (bind _returnvalue (Transformation|GetWorldLocation _spherecomponent))
  ;[1 1 1] Attach on Hit
  (if (not (Variables|Default|GetHasAttached))
    (Transformation|AttachComponentToComponent OtherComp "None" "KeepWorld" "KeepWorld" "KeepWorld" true)
    (Transformation|SetActorLocationAndRotation (+ HitLocation (* HitNormal (Components|Sphere|GetScaledSphereRadius (Variables|Default|GetSphereComponent)))) (Math|Rotator|MakeRotfromZX HitNormal (Transformation|GetActorForwardVector)) false true)
    (Physics|SetSimulatePhysics _spherecomponent false)
    (Audio|PlaySoundatLocation "/Game/Audio/Character/Satchel/Vial_Land_Cue.Vial_Land_Cue" _returnvalue "0, 0, 0" 1.0 1.0 0.0 0 0 0 0)
    (Audio|SpawnSoundAttached "/Game/Audio/Character/Satchel/Vial_Idle_Cue.Vial_Idle_Cue" _spherecomponent "None" "0, 0, 0" "0, 0, 0" "KeepRelativeOffset" true 1.0 1.0 0.0 0 0)
    (Niagara|SpawnSystematLocation "/Game/Art/VFX/FXS_Semtex_Land.FXS_Semtex_Land" _returnvalue (Transformation|GetWorldRotation _spherecomponent))
    (Variables|Default|SetHasAttached true)))

(event EventOnExplode
  (bind _returnvalue (Transformation|GetActorLocation))
  (bind _explosionrange (Variables|Default|GetExplosionRange))
  (Utilities|Visual)
  (Utilities|FlowControl|Sequence
    (:then_0
      (bind (_outactors _returnvalue_2) (Collision|SphereOverlapActors _returnvalue _explosionrange (Utilities|Array|MakeArray "ObjectTypeQuery3") "/Script/GP3.AlchemistCharacter"))
      (if _returnvalue_2
        (bind _returnvalue_3 (Collision|LineTraceByChannel _returnvalue (Transformation|GetActorLocation (Utilities|Array|Get(acopy) _outactors)) "TraceTypeQuery1" false _outactors "None" true "(R=1.000000,G=0.000000,B=0.000000,A=1.000000)" "(R=0.000000,G=1.000000,B=0.000000,A=1.000000)" 1.0))
        (if (not _returnvalue_3)
          (bind _asalchemist_character (Utilities|Casting|CastToAlchemistCharacter (Utilities|Array|Get(acopy) _outactors)))
          (bind _force (CallFunction|CalcForce _asalchemist_character))
          (CallFunction|LaunchPlayer _asalchemist_character _force)
          (Class|AlchemistCharacter|ResetExtraJump _asalchemist_character)
          (Class|AlchemistCharacter|ResetGravity _asalchemist_character)
          (Class|AlchemistCharacter|Boost _asalchemist_character))))
    (:then_1
      (bind _outactors_2 (Collision|SphereOverlapActors _returnvalue _explosionrange (Utilities|Array|MakeArray "ObjectTypeQuery2" "ObjectTypeQuery6") "/Script/GP3.Explodable"))
      (for _array_element _outactors_2
        (bind _asexplodable (Utilities|Casting|CastToExplodable _array_element))
        (Class|Explodable|OnHitbyExplosion _asexplodable self)))
    (:then_2
      (bind _outcomponents (Collision|SphereOverlapComponents _returnvalue _explosionrange (Utilities|Array|MakeArray "ObjectTypeQuery2" "ObjectTypeQuery6" "ObjectTypeQuery1") "/Script/GP3.MeshExplodableComponent"))
      (for _array_element_2 _outcomponents
        (bind _asmesh_explodable_component (Utilities|Casting|CastToMeshExplodableComponent _array_element_2))
        (Class|MeshExplodableComponent|OnHitbyExplosion _asmesh_explodable_component self)))
    (:then_3
      (Actor|DestroyActor))))

(event EventOnDespawn
  ;[1 1 1] Despawn on Player Death
  (Actor|DestroyActor))

(event EventTick
  (params (DeltaSeconds :type Float%20%28single-precision%29))
  (bind _spherecomponent (Variables|Default|GetSphereComponent))
  ;[1 1 1] Additional Gravity
  (if (Physics|IsSimulatingPhysics _spherecomponent "None")
    (Physics|AddForce _spherecomponent (* (Math|Vector|VectorDown) (Variables|Default|GetAdditionalGravity)) "None" true)))

(event EventBeginPlay
  (Utilities|FlowControl|Delay (Variables|Default|GetFuseDuration))
  (bind _asalchemist_character (Utilities|Casting|CastToAlchemistCharacter (Game|GetInstigator)))
  (Class|AbilityComponent|ExplodeBomb (Variables|/Script/GP3.AlchemistCharacter|GetAbilityComponent _asalchemist_character) false))

(fn ConstructionScript)

(fn GetPlayerLocation
  (params (Player :type Alchemist%20Character%20Object%20Reference))
  (bind _returnvalue (Class|AlchemistCharacter|GetGroundLocation Player))
  (bind _returnvalue_2 (Transformation|GetActorLocation Player))
  (bind _returnvalue_3 (Transformation|GetActorLocation))
  (return (select (< (- (.Z (Math|Vector|BreakVector _returnvalue_3)) (.Z (Math|Vector|BreakVector _returnvalue))) 0.0) _returnvalue _returnvalue_2) (Math|Float|Min(Float) (Math|Vector|VectorLength (- _returnvalue_2 _returnvalue_3)) (Math|Vector|VectorLength (- _returnvalue _returnvalue_3)))))

(fn CalcForceOld
  (params (Actor%20location :type Vector))
  (bind _returnvalue (Math|Vector|VectorUp))
  (bind _returnvalue_2 (Transformation|GetActorLocation))
  (bind _launchcurve (Variables|Default|GetLaunchCurve))
  (bind _returnvalue_3 (- Actor%20location _returnvalue_2))
  (bind _returnvalue_4 (Math|Vector|DotProduct _returnvalue_3 _returnvalue))
  (bind _returnvalue_5 (Math|Vector|ProjectVectorontoPlane _returnvalue_3 _returnvalue))
  (bind _returnvalue_6 (Math|Float|Sign(Float) _returnvalue_4))
  (bind _returnvalue_7 (Math|Vector|VectorLength _returnvalue_5))
  (bind _returnvalue_8 (Math|Vector|Normalize _returnvalue_5))
  (bind _returnvalue_9 (* _returnvalue _returnvalue_6))
  (bind _returnvalue_10 (/ _returnvalue_7 1e+03))
  (bind _returnvalue_11 (Math|Curves|GetVectorValue _launchcurve _returnvalue_10))
  (bind (_x _y _z) (Math|Vector|BreakVector _returnvalue_11))
  (bind _returnvalue_12 (Math|Vector|Lerp(Vector) _returnvalue_8 _returnvalue_9 _x))
  (bind _returnvalue_13 (Math|Vector|Normalize _returnvalue_12))
  (Rendering|Debug|DrawDebugArrow _returnvalue_2 (+ (* (* (Variables|Default|GetExplosionRange) _returnvalue_13) _y) _returnvalue_2) 1e+01 (Math|Color|Lerp(LinearColor) "(R=1.000000,G=0.000000,B=0.014251,A=1.000000)" "(R=0.000000,G=0.061501,B=1.000000,A=1.000000)" _z) 5.0 1.0)
  (return (* _returnvalue_13 (* (Variables|Default|GetLaunchForce) _y))))

(fn LaunchPlayer
  (params (Player :type Alchemist%20Character%20Object%20Reference) (New%20Velocity :type Vector))
  (bind _charactermovement (Variables|/Script/Engine.Character|GetCharacterMovement Player))
  (Pawn|Components|CharacterMovement|SetMovementMode _charactermovement "MOVE_Falling" 0)
  (Variables|/Script/Engine.MovementComponent|SetVelocity _charactermovement (Utilities|ChooseMinMaxVectorAddition (Variables|/Script/Engine.MovementComponent|GetVelocity _charactermovement) New%20Velocity))
  (Audio|PlaySoundatLocation "/Game/Audio/Character/Locomotion/Jump/Jump_Start_Fast.Jump_Start_Fast" (Transformation|GetActorLocation Player) "0, 0, 0" 1.0 1.0 0.0 0 0 0 0))

(fn CalcForce
  (params (Player :type Alchemist%20Character%20Object%20Reference))
  (bind _returnvalue (Math|Vector|VectorUp))
  (bind _launchlateralmultiplier (Variables|Default|GetLaunchLateralMultiplier))
  (bind (_location _min_distance) (CallFunction|GetPlayerLocation Player))
  (return (* (* (Math|Vector|Normalize (Math|Vector|SelectVector (Math|Vector|Lerp(Vector) (Math|Vector|Normalize (Math|Vector|ProjectVectorontoPlane (- _location (Transformation|GetActorLocation)) _returnvalue)) (* _returnvalue (Math|Float|Sign(Float) (Math|Vector|DotProduct (- _location (Transformation|GetActorLocation)) _returnvalue))) (.X (Math|Vector|BreakVector (Math|Curves|GetVectorValue (Variables|Default|GetLaunchCurve) (/ (Math|Vector|VectorLength (Math|Vector|ProjectVectorontoPlane (- _location (Transformation|GetActorLocation)) _returnvalue)) 1e+03))))) (- _location (Transformation|GetActorLocation)) (or (< _min_distance (Variables|Default|GetDirectionOverrideThreshold)) (not (AI|Components|NavMovement|IsFalling (Variables|/Script/Engine.Character|GetCharacterMovement Player)))))) (* (Variables|Default|GetLaunchForce) (.Y (Math|Vector|BreakVector (Math|Curves|GetVectorValue (Variables|Default|GetLaunchCurve) (/ (Math|Vector|VectorLength (Math|Vector|ProjectVectorontoPlane (- _location (Transformation|GetActorLocation)) _returnvalue)) 1e+03)))))) (Math|Vector|MakeVector _launchlateralmultiplier _launchlateralmultiplier (Variables|Default|GetLaunchVerticalMultiplier)))))