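; Temporary test actor for a satchel-style explosive that sticks to what it hits and can be detonated to launch the player.
; Hit attaches it to the struck component, keeping world transform.
; Explode notifies nearby Explodable actors found by a fixed-radius sphere overlap, plays effects, then destroys itself.
; The player is launched away from the blast if within ExplosionRange, a separate radius; its debug sphere draw is disconnected.
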(event Custom|Explode
  (bind _returnvalue (Transformation|GetActorLocation))
  (bind _returnvalue_2 (Game|GetPlayerCharacter 0))
  (bind _returnvalue_3 (Transformation|GetActorLocation _returnvalue_2))
  (bind _returnvalue_4 (- _returnvalue_3 _returnvalue))
  (bind _outactors (Collision|SphereOverlapActors (Transformation|GetActorLocation) 5e+02 (Utilities|Array|MakeArray "ObjectTypeQuery2") "/Script/GP3.Explodable"))
  (for _array_element _outactors
    (bind _asexplodable (Utilities|Casting|CastToExplodable _array_element))
    (Class|Explodable|OnHitbyExplosion _asexplodable))
  (Effects|SpawnEmitteratLocation "/Game/StarterContent/Particles/P_Explosion.P_Explosion" (Transformation|GetWorldLocation (Variables|Default|GetCube)))
  (Audio|PlaySound2D "/Game/Audio/Temp_Audio_SatchelExplosion.Temp_Audio_SatchelExplosion" 1.0 1.0 0.0 0 0)
  (if (<= (Math|Vector|VectorLength _returnvalue_4) (Variables|Default|GetExplosionRange))
    (Character|LaunchCharacter _returnvalue_2 (* (Math|Vector|Normalize _returnvalue_4) (Variables|Default|GetLaunchForce)) false false))
  (Actor|DestroyActor))

(event Collision|EventHit
  (params (MyComp :type Primitive%20Component%20Object%20Reference) (Other :type Actor%20Object%20Reference) (OtherComp :type Primitive%20Component%20Object%20Reference) (bSelfMoved :type Boolean) (HitLocation :type Vector :default "0, 0, 0") (HitNormal :type Vector :default "0, 0, 0") (NormalImpulse :type Vector :default "0, 0, 0") (Hit :type Hit%20Result%20Structure%20%28by%20ref%29))
  (Transformation|AttachComponentToComponent OtherComp "None" "KeepWorld" "KeepWorld" "KeepWorld" true))

(fn ConstructionScript)