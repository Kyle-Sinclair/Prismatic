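; Player ability component that lets the owning Character throw, lay, detonate and clear satchel bombs.
; Throws use an eye-level line trace with a yaw-rotated aim offset to aim the launch impulse; lays launch along an actor-relative direction.
; Spawned satchels are queued, and detonation dequeues one to explode.
; Detonation starts a cooldown that ends after a delay only if grounded, otherwise on landing once a short minimum time check passes.
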(event Custom|LandedDelegate_Event
  (params (Hit :type Hit%20Result%20Structure%20%28by%20ref%29))
  ;[1 1 1] Landed Delegate. Clears cooldown
  (Utilities|IsValid (Variables|Default|GetCharacter)
    (:Is%20Valid
      (if (and (> (Class|AbilityComponent|GetBombCooldownTime) 0.1) (Class|AbilityComponent|IsBombCooldown))
        (Class|AbilityComponent|SetBombCooldown false)))))

(event EventOnClearBombQueue
  ;[1 1 1] Clears all bombs in queue
  (for _index (range 0 (Variables|Default|GetMaxBombCount))
    (bind _returnvalue (Class|AbilityComponent|DequeueSpawnedBomb))
    (Utilities|IsValid _returnvalue
      (:Is%20Valid
        (Class|BombActor|Despawn _returnvalue)
        (Math|Integer|DecrementInt (Variables|Default|GetCurrentBombCount))))))

(event EventOnLayBomb
  (bind _character (Variables|Default|GetCharacter))
  (bind _bombspawnoffset (Variables|Default|GetBombSpawnOffset))
  (bind _returnvalue (Transformation|GetActorRotation _character))
  (bind _returnvalue_2 (Transformation|GetActorLocation _character))
  (bind _returnvalue_3 (Math|Vector|GetForwardVector _returnvalue))
  (bind _returnvalue_4 (* _bombspawnoffset _returnvalue_3))
  (bind _returnvalue_5 (+ _returnvalue_4 _returnvalue_2))
  ;[1 1 1] Lay bomb
  (Utilities|ThrowVisual _returnvalue_5)
  (Utilities|SpawnandThrowBomb _returnvalue_5 (Math|Vector|RotateVector (Math|Vector|Normalize (Variables|Default|GetLay%20Direction)) _returnvalue) (Variables|Default|GetBombLayForce)))

(event EventOnThrowBomb
  (bind _returnvalue (Math|Float|MakeLiteralFloat 1e+03))
  (bind _bombspawnoffset (Variables|Default|GetBombSpawnOffset))
  (bind _aimoffset (Variables|Default|GetAimOffset))
  (bind _character (Variables|Default|GetCharacter))
  (bind _returnvalue_2 (Pawn|GetControlRotation _character :!class /Script/Engine.Pawn))
  (bind _returnvalue_3 (Transformation|GetActorRotation _character))
  (bind _outlocation (Actor|GetActorEyesViewPoint _character))
  (bind _returnvalue_4 (Math|Vector|GetForwardVector _returnvalue_2))
  (bind _yaw (Math|Rotator|BreakRotator _returnvalue_2))
  (bind _returnvalue_5 (Math|Vector|GetForwardVector _returnvalue_3))
  (bind _returnvalue_6 (Math|Vector|RotateVectorAroundAxis _aimoffset _yaw "0.000000,0.000000,1.000000"))
  (bind _returnvalue_7 (* _returnvalue_5 _bombspawnoffset))
  (bind _returnvalue_8 (+ _returnvalue_7 _outlocation))
  (bind _returnvalue_9 (+ _returnvalue_4 _returnvalue_6))
  (bind _returnvalue_10 (Math|Vector|Normalize _returnvalue_9))
  (bind _returnvalue_11 (* _returnvalue _returnvalue_10))
  (bind _returnvalue_12 (+ _outlocation _returnvalue_11))
  (Utilities|ThrowVisual _outlocation)
  ;[1 1 1] Perform Ray trace for satchel spawn
  (bind _outhit (Collision|LineTraceByChannel _outlocation _returnvalue_12 "TraceTypeQuery1" true 0 "None"))
  ;[1 1 1] Spawn Satchel and Save Reference to it
  (Utilities|SpawnandThrowBomb _returnvalue_8 (Math|Vector|Normalize (- (select (.bblockinghit _outhit) (.location _outhit) _returnvalue_12) _returnvalue_8)) (Variables|Default|GetBombLaunchForce)))

(event EventOnExplodeBomb
  (bind _character (Variables|Default|GetCharacter))
  ;[1 1 1] Explode Satchel
  (bind _returnvalue (Class|AbilityComponent|DequeueSpawnedBomb))
  (Default|Explode _returnvalue)
  ;[1 1 1] Cooldown for when on ground
  (Class|AbilityComponent|SetBombCooldown true)
  (Utilities|FlowControl|Delay (Variables|Default|GetBombCooldownDuration))
  (Utilities|IsValid _character
    (:Is%20Valid
      (if (not (AI|Components|NavMovement|IsFalling (Variables|/Script/Engine.Character|GetCharacterMovement _character)))
        (Class|AbilityComponent|SetBombCooldown false)))))

(event EventBeginPlay
  ;[1 1 1] Begin Play. Cache player
  (bind _ascharacter (Utilities|Casting|CastToCharacter (Components|GetOwner)))
  (Variables|Default|SetCharacter _ascharacter)
  ;[1 1 1] Landed Delegate. Clears cooldown
  (EventDispatchers|BindEventtoLandedDelegate (Variables|Default|GetCharacter) (delegate Custom|LandedDelegate_Event)))